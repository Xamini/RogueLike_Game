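; Loot drop actor that, on BeginPlay, rolls a rarity and item type, then shows a random helmet or chest plate.
; Weighted rarity sets the stat bonus and color, fed to a dynamic material and the loot widget.
; Interaction events toggle the widget and a custom-depth highlight.
; The item-type switch, including stage-scaled gold spawning in denominations, is disconnected, so every roll yields armor.
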(event Custom|Player_Can_Interact
  (bind _mesh_picked (Variables|Default|GetMesh_Picked))
  (Rendering|SetVisibility (Variables|Default|GetWidget) true false)
  (Variables|Default|SetPlayerCanInteract? true)
  (Rendering|SetRenderCustomDepth _mesh_picked true)
  (Rendering|SetCustomDepthStencilValue _mesh_picked 1))

(event Custom|Choose_Random_Loot
  (bind _rarity_output (CallFunction|ChooseRarity))
  (bind _loot_type (CallFunction|ChooseItemType))
  (bind _output_get (Variables|Default|SetItem_Type _loot_type))
  (CallFunction|ChooseItem _rarity_output _output_get))

(event Custom|End_Surbrillance
  (bind _mesh_picked (Variables|Default|GetMesh_Picked))
  (Rendering|SetVisibility (Variables|Default|GetWidget) false false)
  (Rendering|SetRenderCustomDepth _mesh_picked false)
  (Rendering|SetCustomDepthStencilValue _mesh_picked 0)
  (Variables|Default|SetPlayerCanInteract? false))

(event EventBeginPlay
  (CallFunction|HideMeshes)
  (Rendering|SetVisibility (Variables|Default|GetWidget) false false)
  (CallFunction|ChooseRandomLoot))

(fn ConstructionScript)

(fn ChooseRarity
  (params (Rarity_Chance :type Integer))
  (bind _output_get (LocalVariables|SetRandom_Int (Math|Random|RandomIntegerinRange 1 100)))
  (if (<= _output_get (- 40 Rarity_Chance))
    (return "NewEnumerator0")
    (elif (<= (LocalVariables|GetRandom_Int) (- 70 Rarity_Chance))
      (return "NewEnumerator1")
      (elif (<= (LocalVariables|GetRandom_Int) (- 90 Rarity_Chance))
        (return "NewEnumerator2")
        (else
          (return "NewEnumerator3"))))))

(fn ChooseItemType
  (return (Utilities|Select :Index (Math|Random|RandomIntegerinRange 0 3) :Option%200 "NewEnumerator0" :Option%201 "NewEnumerator1" :Option%202 "NewEnumerator2" :Option%203 "NewEnumerator3")))

(fn ChooseItem
  (params (Rarity :type Rarity_Enum%20Enum :default "NewEnumerator0") (Loot_Type :type LootType_Enum%20Enum :default "NewEnumerator0"))
  (LocalVariables|SetLocal_Rarity Rarity)
  ;[1 1 1] Pick_Armor
  (bind _armor_type (CallFunction|ChooseArmorType))
  (bind _output_get (LocalVariables|SetArmor_Type _armor_type))
  (bind (_statistics_type _stat_level) (CallFunction|ChooseArmorBasicStats (LocalVariables|GetLocal_Rarity) _output_get))
  (bind _output_get_2 (Variables|Default|SetMesh_Picked (.Value (Utilities|Map|Find (Variables|Default|GetMeshes) _armor_type))))
  (Rendering|SetVisibility _output_get_2 true false)
  (bind _asloot_item_widget (Utilities|Casting|CastToLoot_Item_Widget (UserInterface|GetUserWidgetObject (Variables|Default|GetWidget))))
  (Appearance|SetColorandOpacity (Variables|/Game/SpaceRogue/Blueprints/Loot/Loot_Item_Widget.Loot_Item_Widget_C|GetBackground_Color _asloot_item_widget) (Math|Conversions|ToLinearColor(Color) (.Value (Utilities|Map|Find (LocalVariables|GetItem_Color) (LocalVariables|GetLocal_Rarity)))) :!class /Script/UMG.Image)
  (Rendering|Components|TextRender|SetText (Variables|/Game/SpaceRogue/Blueprints/Loot/Loot_Item_Widget.Loot_Item_Widget_C|GetItem_Type_Name _asloot_item_widget) (Utilities|Text|ToText(String) (Utilities|String|EnumtoString _output_get)))
  (Rendering|Components|TextRender|SetText (Variables|/Game/SpaceRogue/Blueprints/Loot/Loot_Item_Widget.Loot_Item_Widget_C|GetPrimary_Stat _asloot_item_widget) (Utilities|Text|ToText(String) (Utilities|String|Append (Utilities|String|EnumtoString _statistics_type) "  +" (Utilities|String|ToString(Integer) _stat_level))))
  (Rendering|Components|TextRender|SetText (Variables|/Game/SpaceRogue/Blueprints/Loot/Loot_Item_Widget.Loot_Item_Widget_C|GetRarity _asloot_item_widget) (Utilities|Text|ToText(String) (Utilities|String|EnumtoString (LocalVariables|GetLocal_Rarity))))
  (bind _values (Utilities|Map|Values (Variables|Default|GetMeshes)))
  (Rendering|Material|SetVectorParameterValue (Utilities|Array|Get(acopy) (Variables|Default|GetMaterial_Instance) (Utilities|Array|FindItem _values (Variables|Default|GetMesh_Picked))) "Item_Color" (Math|Conversions|ToLinearColor(Color) (.Value (Utilities|Map|Find (LocalVariables|GetItem_Color) (LocalVariables|GetLocal_Rarity)))) :!class /Script/Engine.MaterialInstanceDynamic))

(fn ChooseArmorType
  (return (Utilities|Select :Index (Math|Random|RandomIntegerinRange 0 1) :Option%200 "NewEnumerator2" :Option%201 "NewEnumerator3" :Option%202 "NewEnumerator4")))

(fn ChooseArmorBasicStats
  (params (Rarity :type Rarity_Enum%20Enum :default "NewEnumerator0") (Armor_Type :type Armor_Type_Enum%20Enum :default "NewEnumerator2"))
  (return (.Value (Utilities|Map|Find (Variables|Default|GetStat_Type) Armor_Type)) (.Value (Utilities|Map|Find (Variables|Default|GetStat_Level) Rarity))))

(fn HideMeshes
  (Utilities|FlowControl|Sequence
    (:then_0
      (Utilities|Map|Add (Variables|Default|GetMeshes) "NewEnumerator2" (Variables|Default|GetHelmet))
      (Utilities|Map|Add (Variables|Default|GetMeshes) "NewEnumerator3" (Variables|Default|GetChestPlate)))
    (:then_1
      (bind _values (Utilities|Map|Values (Variables|Default|GetMeshes)))
      (for _array_element _values
        (Rendering|SetVisibility _array_element false false)
        (bind _returnvalue (Rendering|Material|CreateDynamicMaterialInstance _array_element 0 "/Game/SpaceRogue/Blueprints/Loot/Rarity_Item_Material_Inst.Rarity_Item_Material_Inst" "None" :!class /Script/Engine.PrimitiveComponent))
        (Utilities|Array|Add (Variables|Default|GetMaterial_Instance) _returnvalue)))))