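; Roguelike loot pickup that rolls a weighted rarity and a helmet or chestplate on BeginPlay, showing its tinted mesh and stat widget data.
; Interaction events toggle the widget and custom-depth highlight.
; Tick polls player interaction, copies stats and color to the matching render actor and player material, then destroys the pickup.
; The rolled item type is ignored: the type switch, including gold spawning, is disconnected, so loot is always armor.
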(event Custom|Player_Can_Interact
  (bind _mesh_picked (Variables|Default|GetMesh_Picked))
  (Rendering|SetVisibility (Variables|Default|GetWidget) true false)
  (Variables|Default|SetPlayerCanInteract? true)
  (Rendering|SetRenderCustomDepth _mesh_picked true)
  (Rendering|SetCustomDepthStencilValue _mesh_picked 1))

(event Custom|Choose_Random_Loot
  (bind _rarity_output (CallFunction|ChooseRarity))
  (bind _loot_type (CallFunction|ChooseItemType))
  (bind _output_get (Variables|Default|SetItem_Type _loot_type))
  (bind (_item_type_name_txt _primary_stat_txt_value _rarity_txt_value _item_color_value) (CallFunction|ChooseItem _rarity_output _output_get))
  (Variables|Default|SetItem_Type_Name _item_type_name_txt)
  (Variables|Default|SetPrimary_Stat_TXT _primary_stat_txt_value)
  (Variables|Default|SetRarity_Txt _rarity_txt_value)
  (Variables|Default|SetItem_Color_Value _item_color_value))

(event Custom|End_Surbrillance
  (bind _mesh_picked (Variables|Default|GetMesh_Picked))
  (Rendering|SetVisibility (Variables|Default|GetWidget) false false)
  (Rendering|SetRenderCustomDepth _mesh_picked false)
  (Rendering|SetCustomDepthStencilValue _mesh_picked 0)
  (Variables|Default|SetPlayerCanInteract? false))

(event EventTick
  (params (DeltaSeconds :type Float%20%28single-precision%29))
  (bind _asplayer_character (Utilities|Casting|CastToPlayer_Character (Game|GetPlayerCharacter 0)))
  (if (Variables|Default|GetPlayerCanInteract?)
    (if (Variables|/Game/RogueLike_Game/Character/Player/Blueprints/Player_Character.Player_Character_C|GetInteract? _asplayer_character)
      (Variables|Default|SetPlayerCanInteract? false)
      (if (Utilities|Enum|Equal(Enum) (Variables|Default|GetArmor_Type) "NewEnumerator2")
        (bind _returnvalue (Actor|GetActorOfClass "/Game/RogueLike_Game/Character/Player/Widgets/Inventaire/Helmet/Helmet_Render_Actor.Helmet_Render_Actor_C"))
        (Rendering|Material|SetVectorParameterValue (Variables|/Game/RogueLike_Game/Character/Player/Widgets/Inventaire/Helmet/Helmet_Render_Actor.Helmet_Render_Actor_C|GetInventory_Dynamic_Material _returnvalue) "Item_Color" (Variables|Default|GetItem_Color_Value) :!class /Script/Engine.MaterialInstanceDynamic)
        (Variables|/Game/RogueLike_Game/Character/Player/Widgets/Inventaire/Helmet/Helmet_Render_Actor.Helmet_Render_Actor_C|SetPrimary_Stat_TXT _returnvalue (Variables|Default|GetPrimary_Stat_TXT))
        (Variables|/Game/RogueLike_Game/Character/Player/Widgets/Inventaire/Helmet/Helmet_Render_Actor.Helmet_Render_Actor_C|SetRarity_Txt _returnvalue (Variables|Default|GetRarity_Txt))
        (Variables|/Game/RogueLike_Game/Character/Player/Widgets/Inventaire/Helmet/Helmet_Render_Actor.Helmet_Render_Actor_C|SetItem_Type_Name _returnvalue (Variables|Default|GetItem_Type_Name))
        (Variables|/Game/RogueLike_Game/Character/Player/Widgets/Inventaire/Helmet/Helmet_Render_Actor.Helmet_Render_Actor_C|SetItem_Color _returnvalue (Variables|Default|GetItem_Color_Value))
        (bind _asplayer_character_2 (Utilities|Casting|CastToPlayer_Character (Game|GetPlayerCharacter 0)))
        (Rendering|Material|SetVectorParameterValue (Variables|/Game/RogueLike_Game/Character/Player/Blueprints/Player_Character.Player_Character_C|GetHelmet_Rarity_Material _asplayer_character_2) "Item_Color" (Variables|Default|GetItem_Color_Value) :!class /Script/Engine.MaterialInstanceDynamic)
        (else
          (bind _returnvalue_2 (Actor|GetActorOfClass "/Game/RogueLike_Game/Character/Player/Widgets/Inventaire/ChestPlate/ChestPlate_Render_Actor.ChestPlate_Render_Actor_C"))
          (Rendering|Material|SetVectorParameterValue (Variables|/Game/RogueLike_Game/Character/Player/Widgets/Inventaire/ChestPlate/ChestPlate_Render_Actor.ChestPlate_Render_Actor_C|GetInventory_Dynamic_Material _returnvalue_2) "Item_Color" (Variables|Default|GetItem_Color_Value) :!class /Script/Engine.MaterialInstanceDynamic)
          (Variables|/Game/RogueLike_Game/Character/Player/Widgets/Inventaire/ChestPlate/ChestPlate_Render_Actor.ChestPlate_Render_Actor_C|SetPrimary_Stat_TXT _returnvalue_2 (Variables|Default|GetPrimary_Stat_TXT))
          (Variables|/Game/RogueLike_Game/Character/Player/Widgets/Inventaire/ChestPlate/ChestPlate_Render_Actor.ChestPlate_Render_Actor_C|SetRarity_Txt _returnvalue_2 (Variables|Default|GetRarity_Txt))
          (Variables|/Game/RogueLike_Game/Character/Player/Widgets/Inventaire/ChestPlate/ChestPlate_Render_Actor.ChestPlate_Render_Actor_C|SetItem_Type_Name _returnvalue_2 (Variables|Default|GetItem_Type_Name))
          (Variables|/Game/RogueLike_Game/Character/Player/Widgets/Inventaire/ChestPlate/ChestPlate_Render_Actor.ChestPlate_Render_Actor_C|SetItem_Color _returnvalue_2 (Variables|Default|GetItem_Color_Value))
          (bind _asplayer_character_3 (Utilities|Casting|CastToPlayer_Character (Game|GetPlayerCharacter 0)))
          (Rendering|Material|SetVectorParameterValue (Variables|/Game/RogueLike_Game/Character/Player/Blueprints/Player_Character.Player_Character_C|GetChestPlate_Rarity_Material _asplayer_character_3) "Item_Color" (Variables|Default|GetItem_Color_Value) :!class /Script/Engine.MaterialInstanceDynamic)))
      (Actor|DestroyActor))))

(event EventBeginPlay
  (CallFunction|HideMeshes)
  (Rendering|SetVisibility (Variables|Default|GetWidget) false false)
  (CallFunction|ChooseRandomLoot))

(fn ConstructionScript)

(fn ChooseRarity
  (params (Rarity_Chance :type Integer))
  (bind _output_get (LocalVariables|SetRandom_Int (Math|Random|RandomIntegerinRange 1 100)))
  (if (<= _output_get (- 40 Rarity_Chance))
    (return "NewEnumerator0")
    (elif (<= (LocalVariables|GetRandom_Int) (- 70 Rarity_Chance))
      (return "NewEnumerator1")
      (elif (<= (LocalVariables|GetRandom_Int) (- 90 Rarity_Chance))
        (return "NewEnumerator2")
        (else
          (return "NewEnumerator3"))))))

(fn ChooseItemType
  (return (Utilities|Select :Index (Math|Random|RandomIntegerinRange 0 3) :Option%200 "NewEnumerator0" :Option%201 "NewEnumerator1" :Option%202 "NewEnumerator2" :Option%203 "NewEnumerator3")))

(fn ChooseItem
  (params (Rarity :type Rarity_Enum%20Enum :default "NewEnumerator0") (Loot_Type :type LootType_Enum%20Enum :default "NewEnumerator0") (InputPin :type Text))
  (LocalVariables|SetLocal_Rarity Rarity)
  ;[1 1 1] Pick_Armor
  (bind _armor_type (CallFunction|ChooseArmorType))
  (bind _output_get (Variables|Default|SetArmor_Type _armor_type))
  (bind (_statistics_type _stat_level) (CallFunction|ChooseArmorBasicStats (LocalVariables|GetLocal_Rarity) _output_get))
  (bind _output_get_2 (Variables|Default|SetMesh_Picked (.Value (Utilities|Map|Find (Variables|Default|GetMeshes) _armor_type))))
  (Rendering|SetVisibility _output_get_2 true false)
  (bind _asloot_item_widget (Utilities|Casting|CastToLoot_Item_Widget (UserInterface|GetUserWidgetObject (Variables|Default|GetWidget))))
  (Appearance|SetColorandOpacity (Variables|/Game/RogueLike_Game/Blueprints/Loot/Loot_Item_Widget.Loot_Item_Widget_C|GetBackground_Color _asloot_item_widget) (Math|Conversions|ToLinearColor(Color) (.Value (Utilities|Map|Find (LocalVariables|GetItem_Color) (LocalVariables|GetLocal_Rarity)))) :!class /Script/UMG.Image)
  (Rendering|Components|TextRender|SetText (Variables|/Game/RogueLike_Game/Blueprints/Loot/Loot_Item_Widget.Loot_Item_Widget_C|GetItem_Type_Name _asloot_item_widget) (Utilities|Text|ToText(String) (Utilities|String|EnumtoString _output_get)))
  (Rendering|Components|TextRender|SetText (Variables|/Game/RogueLike_Game/Blueprints/Loot/Loot_Item_Widget.Loot_Item_Widget_C|GetPrimary_Stat _asloot_item_widget) (Utilities|Text|ToText(String) (Utilities|String|Append (Utilities|String|EnumtoString _statistics_type) "  +" (Utilities|String|ToString(Integer) _stat_level))))
  (Rendering|Components|TextRender|SetText (Variables|/Game/RogueLike_Game/Blueprints/Loot/Loot_Item_Widget.Loot_Item_Widget_C|GetRarity _asloot_item_widget) (Utilities|Text|ToText(String) (Utilities|String|EnumtoString (LocalVariables|GetLocal_Rarity))))
  (bind _values (Utilities|Map|Values (Variables|Default|GetMeshes)))
  (Rendering|Material|SetVectorParameterValue (Utilities|Array|Get(acopy) (Variables|Default|GetMaterial_Instance) (Utilities|Array|FindItem _values (Variables|Default|GetMesh_Picked))) "Item_Color" (Math|Conversions|ToLinearColor(Color) (.Value (Utilities|Map|Find (LocalVariables|GetItem_Color) (LocalVariables|GetLocal_Rarity)))) :!class /Script/Engine.MaterialInstanceDynamic)
  (return (Utilities|Text|ToText(String) (Utilities|String|EnumtoString _output_get)) (Utilities|Text|ToText(String) (Utilities|String|Append (Utilities|String|EnumtoString _statistics_type) "  +" (Utilities|String|ToString(Integer) _stat_level))) (Utilities|Text|ToText(String) (Utilities|String|EnumtoString (LocalVariables|GetLocal_Rarity))) (Math|Conversions|ToLinearColor(Color) (.Value (Utilities|Map|Find (LocalVariables|GetItem_Color) (LocalVariables|GetLocal_Rarity))))))

(fn ChooseArmorType
  (return (Utilities|Select :Index (Math|Random|RandomIntegerinRange 0 1) :Option%200 "NewEnumerator2" :Option%201 "NewEnumerator3" :Option%202 "NewEnumerator4")))

(fn ChooseArmorBasicStats
  (params (Rarity :type Rarity_Enum%20Enum :default "NewEnumerator0") (Armor_Type :type Armor_Type_Enum%20Enum :default "NewEnumerator2"))
  (return (.Value (Utilities|Map|Find (Variables|Default|GetStat_Type) Armor_Type)) (.Value (Utilities|Map|Find (Variables|Default|GetStat_Level) Rarity))))

(fn HideMeshes
  (Utilities|FlowControl|Sequence
    (:then_0
      (Utilities|Map|Add (Variables|Default|GetMeshes) "NewEnumerator2" (Variables|Default|GetHelmet))
      (Utilities|Map|Add (Variables|Default|GetMeshes) "NewEnumerator3" (Variables|Default|GetChestPlate)))
    (:then_1
      (bind _values (Utilities|Map|Values (Variables|Default|GetMeshes)))
      (for _array_element _values
        (Rendering|SetVisibility _array_element false false)
        (bind _returnvalue (Rendering|Material|CreateDynamicMaterialInstance _array_element 0 "/Game/RogueLike_Game/Blueprints/Loot/Rarity_Item_Material_Inst.Rarity_Item_Material_Inst" "None" :!class /Script/Engine.PrimitiveComponent))
        (Utilities|Array|Add (Variables|Default|GetMaterial_Instance) _returnvalue)))))