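; Blacksmith (Forgeron) NPC Blueprint that opens its HUD when the player interacts nearby.
; An interaction box sets a proximity flag and highlights the mesh through custom depth stencil when the player capsule overlaps.
; Tick polls the player's Interact flag through a DoOnce, then adds the HUD and locks movement.
; A timeline blends the player camera to the forge viewpoint, while the player's body and armor meshes hide after a short delay.
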(event OnComponentBeginOverlap(Interactive_Box)
  (params (OverlappedComponent :type Primitive%20Component%20Object%20Reference) (OtherActor :type Actor%20Object%20Reference) (OtherComp :type Primitive%20Component%20Object%20Reference) (OtherBodyIndex :type Integer) (bFromSweep :type Boolean) (SweepResult :type Hit%20Result%20Structure%20%28by%20ref%29))
  (bind _mesh (Variables|Character|GetMesh))
  (if (Components|ComponentHasTag OtherComp "Player_Capsule")
    (Variables|Default|SetPlayerCanInteract? true)
    (Rendering|SetRenderCustomDepth _mesh true)
    (Rendering|SetCustomDepthStencilValue _mesh 1)))

(event OnComponentEndOverlap(Interactive_Box)
  (params (OverlappedComponent :type Primitive%20Component%20Object%20Reference) (OtherActor :type Actor%20Object%20Reference) (OtherComp :type Primitive%20Component%20Object%20Reference) (OtherBodyIndex :type Integer))
  (bind _mesh (Variables|Character|GetMesh))
  (Rendering|SetRenderCustomDepth _mesh false)
  (Rendering|SetCustomDepthStencilValue _mesh 0)
  (Variables|Default|SetPlayerCanInteract? false))

(event Custom|Stop_Camera_Position_Update
  (bind _value (Timeline|Camera_Position_Update Stop)
    (:Update
      (Transformation|SetWorldTransform (Variables|/Game/RogueLike_Game/Character/Player/Blueprints/Player_Character.Player_Character_C|GetCamera (stale EventTick _asplayer_character)) (Math|Transform|Lerp(Transform) (Transformation|GetWorldTransform (Variables|/Game/RogueLike_Game/Character/Player/Blueprints/Player_Character.Player_Character_C|GetCamera (stale EventTick _asplayer_character))) (Transformation|GetWorldTransform (Variables|Default|GetCamera_Position_Forgeron)) _value) false false))))

(event EventTick
  (params (DeltaSeconds :type Float%20%28single-precision%29))
  (bind _mesh (Variables|Character|GetMesh))
  (bind _asplayer_character (Utilities|Casting|CastToPlayer_Character (Game|GetPlayerCharacter 0)))
  (if (Variables|Default|GetPlayerCanInteract?)
    (if (Variables|/Game/RogueLike_Game/Character/Player/Blueprints/Player_Character.Player_Character_C|GetInteract? _asplayer_character)
      (Utilities|FlowControl|DoOnce false :!label _label
        (:Completed
          (Rendering|SetRenderCustomDepth _mesh false)
          (Rendering|SetCustomDepthStencilValue _mesh 0)
          (bind _returnvalue (UserInterface|CreateWidget "/Game/RogueLike_Game/Character/Forgeron/Widgets/HUD_Forgeron.HUD_Forgeron_C"))
          (UserInterface|Viewport|AddtoViewport _returnvalue 0)
          (Variables|/Game/RogueLike_Game/Character/Player/Blueprints/Player_Character.Player_Character_C|SetCan_Move? _asplayer_character false)
          (Utilities|FlowControl|Sequence
            (:then_0
              (bind _value (Timeline|Camera_Position_Update PlayFromStart)
                (:Update
                  (Transformation|SetWorldTransform (Variables|/Game/RogueLike_Game/Character/Player/Blueprints/Player_Character.Player_Character_C|GetCamera _asplayer_character) (Math|Transform|Lerp(Transform) (Transformation|GetWorldTransform (Variables|/Game/RogueLike_Game/Character/Player/Blueprints/Player_Character.Player_Character_C|GetCamera _asplayer_character)) (Transformation|GetWorldTransform (Variables|Default|GetCamera_Position_Forgeron)) _value) false false))))
            (:then_1
              (Utilities|FlowControl|Delay 0.5)
              (Rendering|SetVisibility (Variables|/Script/Engine.Character|GetMesh _asplayer_character) false false)))))
      (else
        (goto _label Reset)))))

(fn ConstructionScript)