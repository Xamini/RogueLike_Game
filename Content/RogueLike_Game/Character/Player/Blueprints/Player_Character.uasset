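; Player character for a roguelike, handling diagonal-axis movement, cursor-facing rotation outside the hub, inventory toggling and interaction input.
; An overlay map drives a separate MapMenu_CameraActor for panning, zooming, recentering and snapping, with movement inputs redirected while open.
; Map teleport shows a brief HUD, then moves the capsule to the selected component.
; Tick prints debug stats and sphere-traces ahead to highlight loot actors through a DoOnce gate.
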(event Custom|Teleport_From_Map
  ;[1 1 1] Map_Teleportation
  (Widget|RemovefromParent (Variables|Default|GetMapMenu_Widget))
  (Variables|Default|SetMapMenu%20Open? false)
  (Utilities|FlowControl|Sequence
    (:then_0
      (Utilities|FlowControl|Delay 0.1)
      (bind _returnvalue (UserInterface|CreateWidget "/Game/RogueLike_Game/Character/Player/Widgets/Teleport_HUD.Teleport_HUD_C"))
      (UserInterface|Viewport|AddtoViewport _returnvalue 0)
      (Utilities|FlowControl|Delay 0.75)
      (Widget|RemovefromParent _returnvalue))
    (:then_1
      (Utilities|FlowControl|Delay 0.2)
      (bind _outactors (Actor|GetAllActorsOfClass "/Game/RogueLike_Game/Character/Player/Widgets/MapMenu/MapMenu_CameraActor.MapMenu_CameraActor_C"))
      (Rendering|SetCustomDepthStencilValue (Variables|/Game/RogueLike_Game/Character/Player/Widgets/MapMenu/MapMenu_CameraActor.MapMenu_CameraActor_C|GetCurrent_Hit_Component (Utilities|Array|Get(acopy) _outactors)) (Variables|/Game/RogueLike_Game/Character/Player/Widgets/MapMenu/MapMenu_CameraActor.MapMenu_CameraActor_C|GetCurrent_Stencil_Value_Component (Utilities|Array|Get(acopy) _outactors)))
      (Transformation|SetWorldLocation (Variables|Collision|GetCapsuleComponent) (Math|Vector|MakeVector (.x (Transformation|GetWorldLocation (Variables|/Game/RogueLike_Game/Character/Player/Widgets/MapMenu/MapMenu_CameraActor.MapMenu_CameraActor_C|GetCurrent_Hit_Component (Utilities|Array|Get(acopy) _outactors)))) (.y (Transformation|GetWorldLocation (Variables|/Game/RogueLike_Game/Character/Player/Widgets/MapMenu/MapMenu_CameraActor.MapMenu_CameraActor_C|GetCurrent_Hit_Component (Utilities|Array|Get(acopy) _outactors)))) 95.0) false false))))

(event EventTick
  (params (DeltaSeconds :type Float%20%28single-precision%29))
  (bind _returnvalue (Game|GetPlayerCharacter 0))
  (bind _returnvalue_2 (Transformation|GetActorLocation _returnvalue))
  (Development|PrintString (Utilities|String|Append "Health Point : " (Utilities|String|ToString(Integer) (Variables|Statistics|GetHealthPoint))) true true "(R=0.000000,G=0.660000,B=1.000000,A=1.000000)" 0.0)
  (Development|PrintString (Utilities|String|Append "Max Health Point : " (Utilities|String|ToString(Integer) (Variables|Statistics|GetMax_HealthPoint))) true true "(R=0.000000,G=0.660000,B=1.000000,A=1.000000)" 0.0)
  (Development|PrintString (Utilities|String|Append "Dash Cooldown : " (Utilities|String|ToString(Float) (Variables|Statistics|GetDash_Cooldown))) true true "(R=0.000000,G=0.660000,B=1.000000,A=1.000000)" 0.0)
  (Development|PrintString (Utilities|String|Append "Dash Amount : " (Utilities|String|ToString(Integer) (Variables|Statistics|GetDash_Amount))) true true "(R=0.000000,G=0.660000,B=1.000000,A=1.000000)" 0.0)
  (Development|PrintString (Utilities|String|Append "Fortune : " (Utilities|String|ToString(Float) (Variables|Statistics|GetFortune))) true true "(R=0.000000,G=0.660000,B=1.000000,A=1.000000)" 0.0)
  (Development|PrintString (Utilities|String|Append "Gold : " (Utilities|String|ToString(Integer) (Variables|Statistics|GetGold))) true true "(R=0.000000,G=0.660000,B=1.000000,A=1.000000)" 0.0)
  (bind _outhit (Collision|SphereTraceByChannel _returnvalue_2 (+ _returnvalue_2 (* (Math|Vector|GetForwardVector (Variables|Collision|GetCapsuleComponent)) 2e+02)) 5e+01 "TraceTypeQuery1" false 0 "None" true "(R=1.000000,G=0.000000,B=0.000000,A=1.000000)" "(R=0.000000,G=1.000000,B=0.000000,A=1.000000)" 1.0))
  (if (.bBlockingHit (Collision|BreakHitResult _outhit))
    (Utilities|FlowControl|DoOnce false :!label _label
      (:Completed
        (bind _output_get (Variables|Default|SetCurrent_Hited_Actor (Components|GetOwner (.HitComponent (Collision|BreakHitResult _outhit)))))
        (if (Actor|ActorHasTag (Components|GetOwner (.HitComponent (Collision|BreakHitResult _outhit))) "ItemActor")
          (bind _asloot_system_actor (Utilities|Casting|CastToLoot_System_Actor _output_get))
          (Default|PlayerCanInteract _asloot_system_actor))))
    (else
      (bind _asloot_system_actor_2 (Utilities|Casting|CastToLoot_System_Actor (Variables|Default|GetCurrent_Hited_Actor))
        (:then
          (Utilities|IsValid _asloot_system_actor_2
            (:Is%20Valid
              (Default|EndSurbrillance _asloot_system_actor_2)
              (goto _label Reset))
            (:Is%20Not%20Valid
              (goto _label Reset))))
        (:CastFailed
          (goto _label Reset))))))

(event Input|ActionEvents|InputActionOpen_MapMenu
  (params (Key :type Key%20Structure :default "None"))
  (bind _returnvalue (Transformation|GetActorLocation))
  ;[1 1 1] Open_Map
  (:Pressed
    (if (not (Variables|Default|GetIs%20in%20HUB?))
      (if (Variables|Default|GetMapMenu%20Open?)
        (bind _outactors (Actor|GetAllActorsOfClass "/Game/RogueLike_Game/Character/Player/Widgets/MapMenu/MapMenu_CameraActor.MapMenu_CameraActor_C"))
        (Rendering|SetCustomDepthStencilValue (Variables|/Game/RogueLike_Game/Character/Player/Widgets/MapMenu/MapMenu_CameraActor.MapMenu_CameraActor_C|GetCurrent_Hit_Component (Utilities|Array|Get(acopy) _outactors)) (Variables|/Game/RogueLike_Game/Character/Player/Widgets/MapMenu/MapMenu_CameraActor.MapMenu_CameraActor_C|GetCurrent_Stencil_Value_Component (Utilities|Array|Get(acopy) _outactors)))
        (Widget|RemovefromParent (Variables|Default|GetMapMenu_Widget))
        (Variables|Default|SetMapMenu%20Open? false)
        (else
          (bind _returnvalue_2 (UserInterface|CreateWidget "/Game/RogueLike_Game/Character/Player/Widgets/MapMenu/MapMenu_Widget.MapMenu_Widget_C"))
          (bind _output_get (Variables|Default|SetMapMenu_Widget _returnvalue_2))
          (UserInterface|Viewport|AddtoViewport _output_get 0)
          (Variables|Default|SetMapMenu%20Open? true)
          (bind _outactors_2 (Actor|GetAllActorsOfClass "/Game/RogueLike_Game/Character/Player/Widgets/MapMenu/MapMenu_CameraActor.MapMenu_CameraActor_C"))
          (Transformation|SetWorldLocation (Variables|/Game/RogueLike_Game/Character/Player/Widgets/MapMenu/MapMenu_CameraActor.MapMenu_CameraActor_C|GetDefaultSceneRoot (Utilities|Array|Get(acopy) _outactors_2)) (Math|Vector|MakeVector (.x _returnvalue) (.y _returnvalue) 0.0) false false))))))

(event Input|ActionEvents|InputActionInteraction
  (params (Key :type Key%20Structure :default "None"))
  (:Pressed
    (Variables|Default|SetInteract? true))
  (:Released
    (Variables|Default|SetInteract? false)))

(event Input|ActionEvents|InputActionInventory_Menu
  (params (Key :type Key%20Structure :default "None"))
  (:Pressed
    (if (Variables|Default|GetInventory_Open?)
      (Widget|RemovefromParent (stale _returnvalue))
      (Variables|Default|SetInventory_Open? false)
      (else
        (bind _returnvalue (UserInterface|CreateWidget "/Game/RogueLike_Game/Character/Player/Widgets/Inventaire/Inventory_Widget.Inventory_Widget_C"))
        (UserInterface|Viewport|AddtoViewport _returnvalue 0)
        (Variables|Default|SetInventory_Open? true)))))

(event Input|ActionEvents|InputActionRecenter_Map_Menu
  (params (Key :type Key%20Structure :default "None"))
  (bind _returnvalue (Transformation|GetActorLocation))
  ;[1 1 1] Recenter_MapMenu
  (:Pressed
    (if (Variables|Default|GetMapMenu%20Open?)
      (bind _outactors (Actor|GetAllActorsOfClass "/Game/RogueLike_Game/Character/Player/Widgets/MapMenu/MapMenu_CameraActor.MapMenu_CameraActor_C"))
      (Transformation|SetWorldLocation (Variables|/Game/RogueLike_Game/Character/Player/Widgets/MapMenu/MapMenu_CameraActor.MapMenu_CameraActor_C|GetDefaultSceneRoot (Utilities|Array|Get(acopy) _outactors)) (Math|Vector|MakeVector (.x _returnvalue) (.y _returnvalue) 0.0) false false))))

(event Input|AxisEvents|InputAxisMoveForward
  (params (AxisValue :type Float%20%28single-precision%29))
  (bind _returnvalue (* AxisValue 1e+02))
  (if (Variables|Default|GetMapMenu%20Open?)
    (CallFunction|MoveMapMenuXAxis AxisValue)
    (else
      (Pawn|Input|AddMovementInput (Math|Vector|MakeVector _returnvalue _returnvalue 0.0) 1.0 false)
      (CallFunction|CharacterLookatCursor))))

(event Input|AxisEvents|InputAxisMoveRight
  (params (AxisValue :type Float%20%28single-precision%29))
  (bind _returnvalue (* AxisValue 1e+02))
  (if (Variables|Default|GetMapMenu%20Open?)
    (CallFunction|MoveMapMenuYAxis AxisValue)
    (else
      (Pawn|Input|AddMovementInput (Math|Vector|MakeVector (* _returnvalue -1.0) _returnvalue 0.0) 1.0 false)
      (CallFunction|CharacterLookatCursor))))

(event Input|AxisEvents|InputAxisLeftClick_Hold
  (params (AxisValue :type Float%20%28single-precision%29))
  (bind _returnvalue (Class|Actor|GetInputAxisKeyValue))
  (bind _returnvalue_2 (Class|Actor|GetInputAxisKeyValue))
  ;[1 1 1] Drag MapMenu
  (if (Variables|Default|GetMapMenu%20Open?)
    (bind _outactors (Actor|GetAllActorsOfClass "/Game/RogueLike_Game/Character/Player/Widgets/MapMenu/MapMenu_CameraActor.MapMenu_CameraActor_C"))
    (if (> _returnvalue 0.0)
      (Transformation|SetWorldLocation (Variables|/Game/RogueLike_Game/Character/Player/Widgets/MapMenu/MapMenu_CameraActor.MapMenu_CameraActor_C|GetDefaultSceneRoot (Utilities|Array|Get(acopy) _outactors)) (Math|Vector|MakeVector (+ (.x (Transformation|GetWorldLocation (Variables|/Game/RogueLike_Game/Character/Player/Widgets/MapMenu/MapMenu_CameraActor.MapMenu_CameraActor_C|GetDefaultSceneRoot (Utilities|Array|Get(acopy) _outactors)))) (* (/ (Variables|/Script/Engine.SceneCaptureComponent2D|GetOrthoWidth (Variables|/Game/RogueLike_Game/Character/Player/Widgets/MapMenu/MapMenu_CameraActor.MapMenu_CameraActor_C|GetMapMenu_ComponentCapture (Utilities|Array|Get(acopy) _outactors))) 1e+02) (* (Math|Float|Absolute(Float) _returnvalue) -1.0))) (+ (.y (Transformation|GetWorldLocation (Variables|/Game/RogueLike_Game/Character/Player/Widgets/MapMenu/MapMenu_CameraActor.MapMenu_CameraActor_C|GetDefaultSceneRoot (Utilities|Array|Get(acopy) _outactors)))) (* (/ (Variables|/Script/Engine.SceneCaptureComponent2D|GetOrthoWidth (Variables|/Game/RogueLike_Game/Character/Player/Widgets/MapMenu/MapMenu_CameraActor.MapMenu_CameraActor_C|GetMapMenu_ComponentCapture (Utilities|Array|Get(acopy) _outactors))) 1e+02) (* (Math|Float|Absolute(Float) _returnvalue) -1.0))) 0.0) false false)
      (elif (< _returnvalue 0.0)
        (Transformation|SetWorldLocation (Variables|/Game/RogueLike_Game/Character/Player/Widgets/MapMenu/MapMenu_CameraActor.MapMenu_CameraActor_C|GetDefaultSceneRoot (Utilities|Array|Get(acopy) _outactors)) (Math|Vector|MakeVector (- (.x (Transformation|GetWorldLocation (Variables|/Game/RogueLike_Game/Character/Player/Widgets/MapMenu/MapMenu_CameraActor.MapMenu_CameraActor_C|GetDefaultSceneRoot (Utilities|Array|Get(acopy) _outactors)))) (* (/ (Variables|/Script/Engine.SceneCaptureComponent2D|GetOrthoWidth (Variables|/Game/RogueLike_Game/Character/Player/Widgets/MapMenu/MapMenu_CameraActor.MapMenu_CameraActor_C|GetMapMenu_ComponentCapture (Utilities|Array|Get(acopy) _outactors))) 1e+02) (* (Math|Float|Absolute(Float) _returnvalue) -1.0))) (- (.y (Transformation|GetWorldLocation (Variables|/Game/RogueLike_Game/Character/Player/Widgets/MapMenu/MapMenu_CameraActor.MapMenu_CameraActor_C|GetDefaultSceneRoot (Utilities|Array|Get(acopy) _outactors)))) (* (/ (Variables|/Script/Engine.SceneCaptureComponent2D|GetOrthoWidth (Variables|/Game/RogueLike_Game/Character/Player/Widgets/MapMenu/MapMenu_CameraActor.MapMenu_CameraActor_C|GetMapMenu_ComponentCapture (Utilities|Array|Get(acopy) _outactors))) 1e+02) (* (Math|Float|Absolute(Float) _returnvalue) -1.0))) 0.0) false false)))
    (if (< _returnvalue_2 0.0)
      (Transformation|SetWorldLocation (Variables|/Game/RogueLike_Game/Character/Player/Widgets/MapMenu/MapMenu_CameraActor.MapMenu_CameraActor_C|GetDefaultSceneRoot (Utilities|Array|Get(acopy) _outactors)) (Math|Vector|MakeVector (- (.x (Transformation|GetWorldLocation (Variables|/Game/RogueLike_Game/Character/Player/Widgets/MapMenu/MapMenu_CameraActor.MapMenu_CameraActor_C|GetDefaultSceneRoot (Utilities|Array|Get(acopy) _outactors)))) (* (/ (Variables|/Script/Engine.SceneCaptureComponent2D|GetOrthoWidth (Variables|/Game/RogueLike_Game/Character/Player/Widgets/MapMenu/MapMenu_CameraActor.MapMenu_CameraActor_C|GetMapMenu_ComponentCapture (Utilities|Array|Get(acopy) _outactors))) 1e+02) (Math|Float|Absolute(Float) _returnvalue_2))) (+ (.y (Transformation|GetWorldLocation (Variables|/Game/RogueLike_Game/Character/Player/Widgets/MapMenu/MapMenu_CameraActor.MapMenu_CameraActor_C|GetDefaultSceneRoot (Utilities|Array|Get(acopy) _outactors)))) (* (/ (Variables|/Script/Engine.SceneCaptureComponent2D|GetOrthoWidth (Variables|/Game/RogueLike_Game/Character/Player/Widgets/MapMenu/MapMenu_CameraActor.MapMenu_CameraActor_C|GetMapMenu_ComponentCapture (Utilities|Array|Get(acopy) _outactors))) 1e+02) (Math|Float|Absolute(Float) _returnvalue_2))) 0.0) false false)
      (elif (> _returnvalue_2 0.0)
        (Transformation|SetWorldLocation (Variables|/Game/RogueLike_Game/Character/Player/Widgets/MapMenu/MapMenu_CameraActor.MapMenu_CameraActor_C|GetDefaultSceneRoot (Utilities|Array|Get(acopy) _outactors)) (Math|Vector|MakeVector (+ (.x (Transformation|GetWorldLocation (Variables|/Game/RogueLike_Game/Character/Player/Widgets/MapMenu/MapMenu_CameraActor.MapMenu_CameraActor_C|GetDefaultSceneRoot (Utilities|Array|Get(acopy) _outactors)))) (* (/ (Variables|/Script/Engine.SceneCaptureComponent2D|GetOrthoWidth (Variables|/Game/RogueLike_Game/Character/Player/Widgets/MapMenu/MapMenu_CameraActor.MapMenu_CameraActor_C|GetMapMenu_ComponentCapture (Utilities|Array|Get(acopy) _outactors))) 1e+02) (Math|Float|Absolute(Float) _returnvalue_2))) (- (.y (Transformation|GetWorldLocation (Variables|/Game/RogueLike_Game/Character/Player/Widgets/MapMenu/MapMenu_CameraActor.MapMenu_CameraActor_C|GetDefaultSceneRoot (Utilities|Array|Get(acopy) _outactors)))) (* (/ (Variables|/Script/Engine.SceneCaptureComponent2D|GetOrthoWidth (Variables|/Game/RogueLike_Game/Character/Player/Widgets/MapMenu/MapMenu_CameraActor.MapMenu_CameraActor_C|GetMapMenu_ComponentCapture (Utilities|Array|Get(acopy) _outactors))) 1e+02) (Math|Float|Absolute(Float) _returnvalue_2))) 0.0) false false)))))

(event Input|GamepadEvents|GamepadRightTriggerAxis
  (params (AxisValue :type Float%20%28single-precision%29))
  ;[1 1 1] Zoom In/Out MapMenu
  (if (> AxisValue 0.0)
    (if (Variables|Default|GetMapMenu%20Open?)
      (bind _outactors (Actor|GetAllActorsOfClass "/Game/RogueLike_Game/Character/Player/Widgets/MapMenu/MapMenu_CameraActor.MapMenu_CameraActor_C"))
      (if (> (Variables|/Script/Engine.SceneCaptureComponent2D|GetOrthoWidth (Variables|/Game/RogueLike_Game/Character/Player/Widgets/MapMenu/MapMenu_CameraActor.MapMenu_CameraActor_C|GetMapMenu_ComponentCapture (Utilities|Array|Get(acopy) _outactors))) (Variables|Default|GetMin_MapMenu_Zoom))
        (Variables|/Script/Engine.SceneCaptureComponent2D|SetOrthoWidth (Variables|/Game/RogueLike_Game/Character/Player/Widgets/MapMenu/MapMenu_CameraActor.MapMenu_CameraActor_C|GetMapMenu_ComponentCapture (Utilities|Array|Get(acopy) _outactors)) (- (Variables|/Script/Engine.SceneCaptureComponent2D|GetOrthoWidth (Variables|/Game/RogueLike_Game/Character/Player/Widgets/MapMenu/MapMenu_CameraActor.MapMenu_CameraActor_C|GetMapMenu_ComponentCapture (Utilities|Array|Get(acopy) _outactors))) 5e+03))
        (Variables|/Script/Engine.SceneCaptureComponent2D|SetOrthoWidth (Variables|/Game/RogueLike_Game/Character/Player/Widgets/MapMenu/MapMenu_CameraActor.MapMenu_CameraActor_C|GetMapMenu_ComponentCapture_Opacity (Utilities|Array|Get(acopy) _outactors)) (- (Variables|/Script/Engine.SceneCaptureComponent2D|GetOrthoWidth (Variables|/Game/RogueLike_Game/Character/Player/Widgets/MapMenu/MapMenu_CameraActor.MapMenu_CameraActor_C|GetMapMenu_ComponentCapture_Opacity (Utilities|Array|Get(acopy) _outactors))) 1e+03))))))

(event Input|GamepadEvents|GamepadLeftTriggerAxis
  (params (AxisValue :type Float%20%28single-precision%29))
  ;[1 1 1] Zoom In/Out MapMenu
  (if (> AxisValue 0.0)
    (if (Variables|Default|GetMapMenu%20Open?)
      (bind _outactors (Actor|GetAllActorsOfClass "/Game/RogueLike_Game/Character/Player/Widgets/MapMenu/MapMenu_CameraActor.MapMenu_CameraActor_C"))
      (if (< (Variables|/Script/Engine.SceneCaptureComponent2D|GetOrthoWidth (Variables|/Game/RogueLike_Game/Character/Player/Widgets/MapMenu/MapMenu_CameraActor.MapMenu_CameraActor_C|GetMapMenu_ComponentCapture (Utilities|Array|Get(acopy) _outactors))) (Variables|Default|GetMax_MapMenu_Zoom))
        (Variables|/Script/Engine.SceneCaptureComponent2D|SetOrthoWidth (Variables|/Game/RogueLike_Game/Character/Player/Widgets/MapMenu/MapMenu_CameraActor.MapMenu_CameraActor_C|GetMapMenu_ComponentCapture (Utilities|Array|Get(acopy) _outactors)) (+ (Variables|/Script/Engine.SceneCaptureComponent2D|GetOrthoWidth (Variables|/Game/RogueLike_Game/Character/Player/Widgets/MapMenu/MapMenu_CameraActor.MapMenu_CameraActor_C|GetMapMenu_ComponentCapture (Utilities|Array|Get(acopy) _outactors))) 5e+03))
        (Variables|/Script/Engine.SceneCaptureComponent2D|SetOrthoWidth (Variables|/Game/RogueLike_Game/Character/Player/Widgets/MapMenu/MapMenu_CameraActor.MapMenu_CameraActor_C|GetMapMenu_ComponentCapture_Opacity (Utilities|Array|Get(acopy) _outactors)) (+ (Variables|/Script/Engine.SceneCaptureComponent2D|GetOrthoWidth (Variables|/Game/RogueLike_Game/Character/Player/Widgets/MapMenu/MapMenu_CameraActor.MapMenu_CameraActor_C|GetMapMenu_ComponentCapture_Opacity (Utilities|Array|Get(acopy) _outactors))) 1e+03))))))

(event Input|MouseEvents|LeftMouseButton
  (params (Key :type Key%20Structure :default "None"))
  ;[1 1 1] Snap_Map
  (:Released
    (if (Variables|Default|GetMapMenu%20Open?)
      (bind _outactors (Actor|GetAllActorsOfClass "/Game/RogueLike_Game/Character/Player/Widgets/MapMenu/MapMenu_CameraActor.MapMenu_CameraActor_C"))
      (bind _value (Timeline|Snap_Map_Interpolate PlayFromStart)
        (:Update
          (Transformation|SetWorldLocation (Variables|/Game/RogueLike_Game/Character/Player/Widgets/MapMenu/MapMenu_CameraActor.MapMenu_CameraActor_C|GetDefaultSceneRoot (Utilities|Array|Get(acopy) _outactors)) (Math|Vector|MakeVector (Math|Float|Lerp (.x (Transformation|GetWorldLocation (Variables|/Game/RogueLike_Game/Character/Player/Widgets/MapMenu/MapMenu_CameraActor.MapMenu_CameraActor_C|GetDefaultSceneRoot (Utilities|Array|Get(acopy) _outactors)))) (.x (Transformation|GetWorldLocation (Variables|/Game/RogueLike_Game/Character/Player/Widgets/MapMenu/MapMenu_CameraActor.MapMenu_CameraActor_C|GetCurrent_Hit_Component (Utilities|Array|Get(acopy) _outactors)))) _value) (Math|Float|Lerp (.y (Transformation|GetWorldLocation (Variables|/Game/RogueLike_Game/Character/Player/Widgets/MapMenu/MapMenu_CameraActor.MapMenu_CameraActor_C|GetDefaultSceneRoot (Utilities|Array|Get(acopy) _outactors)))) (.y (Transformation|GetWorldLocation (Variables|/Game/RogueLike_Game/Character/Player/Widgets/MapMenu/MapMenu_CameraActor.MapMenu_CameraActor_C|GetCurrent_Hit_Component (Utilities|Array|Get(acopy) _outactors)))) _value) 0.0) false false))))))

(event Input|MouseEvents|MouseWheelUp
  (params (Key :type Key%20Structure :default "None"))
  ;[1 1 1] Zoom In/Out MapMenu
  (:Pressed
    (if (Variables|Default|GetMapMenu%20Open?)
      (bind _outactors (Actor|GetAllActorsOfClass "/Game/RogueLike_Game/Character/Player/Widgets/MapMenu/MapMenu_CameraActor.MapMenu_CameraActor_C"))
      (if (> (Variables|/Script/Engine.SceneCaptureComponent2D|GetOrthoWidth (Variables|/Game/RogueLike_Game/Character/Player/Widgets/MapMenu/MapMenu_CameraActor.MapMenu_CameraActor_C|GetMapMenu_ComponentCapture (Utilities|Array|Get(acopy) _outactors))) (Variables|Default|GetMin_MapMenu_Zoom))
        (Variables|/Script/Engine.SceneCaptureComponent2D|SetOrthoWidth (Variables|/Game/RogueLike_Game/Character/Player/Widgets/MapMenu/MapMenu_CameraActor.MapMenu_CameraActor_C|GetMapMenu_ComponentCapture (Utilities|Array|Get(acopy) _outactors)) (- (Variables|/Script/Engine.SceneCaptureComponent2D|GetOrthoWidth (Variables|/Game/RogueLike_Game/Character/Player/Widgets/MapMenu/MapMenu_CameraActor.MapMenu_CameraActor_C|GetMapMenu_ComponentCapture (Utilities|Array|Get(acopy) _outactors))) 5e+03))
        (Variables|/Script/Engine.SceneCaptureComponent2D|SetOrthoWidth (Variables|/Game/RogueLike_Game/Character/Player/Widgets/MapMenu/MapMenu_CameraActor.MapMenu_CameraActor_C|GetMapMenu_ComponentCapture_Opacity (Utilities|Array|Get(acopy) _outactors)) (- (Variables|/Script/Engine.SceneCaptureComponent2D|GetOrthoWidth (Variables|/Game/RogueLike_Game/Character/Player/Widgets/MapMenu/MapMenu_CameraActor.MapMenu_CameraActor_C|GetMapMenu_ComponentCapture_Opacity (Utilities|Array|Get(acopy) _outactors))) 1e+03))))))

(event Input|MouseEvents|MouseWheelDown
  (params (Key :type Key%20Structure :default "None"))
  ;[1 1 1] Zoom In/Out MapMenu
  (:Pressed
    (if (Variables|Default|GetMapMenu%20Open?)
      (bind _outactors (Actor|GetAllActorsOfClass "/Game/RogueLike_Game/Character/Player/Widgets/MapMenu/MapMenu_CameraActor.MapMenu_CameraActor_C"))
      (if (< (Variables|/Script/Engine.SceneCaptureComponent2D|GetOrthoWidth (Variables|/Game/RogueLike_Game/Character/Player/Widgets/MapMenu/MapMenu_CameraActor.MapMenu_CameraActor_C|GetMapMenu_ComponentCapture (Utilities|Array|Get(acopy) _outactors))) (Variables|Default|GetMax_MapMenu_Zoom))
        (Variables|/Script/Engine.SceneCaptureComponent2D|SetOrthoWidth (Variables|/Game/RogueLike_Game/Character/Player/Widgets/MapMenu/MapMenu_CameraActor.MapMenu_CameraActor_C|GetMapMenu_ComponentCapture (Utilities|Array|Get(acopy) _outactors)) (+ (Variables|/Script/Engine.SceneCaptureComponent2D|GetOrthoWidth (Variables|/Game/RogueLike_Game/Character/Player/Widgets/MapMenu/MapMenu_CameraActor.MapMenu_CameraActor_C|GetMapMenu_ComponentCapture (Utilities|Array|Get(acopy) _outactors))) 5e+03))
        (Variables|/Script/Engine.SceneCaptureComponent2D|SetOrthoWidth (Variables|/Game/RogueLike_Game/Character/Player/Widgets/MapMenu/MapMenu_CameraActor.MapMenu_CameraActor_C|GetMapMenu_ComponentCapture_Opacity (Utilities|Array|Get(acopy) _outactors)) (+ (Variables|/Script/Engine.SceneCaptureComponent2D|GetOrthoWidth (Variables|/Game/RogueLike_Game/Character/Player/Widgets/MapMenu/MapMenu_CameraActor.MapMenu_CameraActor_C|GetMapMenu_ComponentCapture_Opacity (Utilities|Array|Get(acopy) _outactors))) 1e+03))))))

(event Input|GamepadEvents|GamepadFaceButtonRight
  (params (Key :type Key%20Structure :default "None"))
  ;[1 1 1] Open_Map
  (:Pressed
    (if (Variables|Default|GetMapMenu%20Open?)
      (bind _outactors (Actor|GetAllActorsOfClass "/Game/RogueLike_Game/Character/Player/Widgets/MapMenu/MapMenu_CameraActor.MapMenu_CameraActor_C"))
      (Rendering|SetCustomDepthStencilValue (Variables|/Game/RogueLike_Game/Character/Player/Widgets/MapMenu/MapMenu_CameraActor.MapMenu_CameraActor_C|GetCurrent_Hit_Component (Utilities|Array|Get(acopy) _outactors)) (Variables|/Game/RogueLike_Game/Character/Player/Widgets/MapMenu/MapMenu_CameraActor.MapMenu_CameraActor_C|GetCurrent_Stencil_Value_Component (Utilities|Array|Get(acopy) _outactors)))
      (Widget|RemovefromParent (Variables|Default|GetMapMenu_Widget))
      (Variables|Default|SetMapMenu%20Open? false))))

(fn ConstructionScript)

(fn CharacterLookatCursor
  (if (not (Variables|Default|GetIs%20in%20HUB?))
    (Transformation|SetWorldRotation (Variables|Collision|GetCapsuleComponent) (Math|Rotator|MakeRotator 0.0 0.0 (.yaw (Math|Rotator|FindLookatRotation (Transformation|GetActorLocation self) (.Location (Collision|BreakHitResult (.HitResult (Game|Player|GetHitResultUnderCursorbyChannel (Game|GetPlayerController 0) "TraceTypeQuery1" true))))))) false false)))

(fn MoveMapMenuXAxis
  (params (Axis_X_Value :type Float%20%28single-precision%29))
  (bind _outactors (Actor|GetAllActorsOfClass "/Game/RogueLike_Game/Character/Player/Widgets/MapMenu/MapMenu_CameraActor.MapMenu_CameraActor_C"))
  (if (> Axis_X_Value 0.0)
    (Transformation|SetWorldLocation (Variables|/Game/RogueLike_Game/Character/Player/Widgets/MapMenu/MapMenu_CameraActor.MapMenu_CameraActor_C|GetDefaultSceneRoot (Utilities|Array|Get(acopy) _outactors)) (Math|Vector|MakeVector (+ (.x (Transformation|GetWorldLocation (Variables|/Game/RogueLike_Game/Character/Player/Widgets/MapMenu/MapMenu_CameraActor.MapMenu_CameraActor_C|GetDefaultSceneRoot (Utilities|Array|Get(acopy) _outactors)))) (/ (Variables|/Script/Engine.SceneCaptureComponent2D|GetOrthoWidth (Variables|/Game/RogueLike_Game/Character/Player/Widgets/MapMenu/MapMenu_CameraActor.MapMenu_CameraActor_C|GetMapMenu_ComponentCapture (Utilities|Array|Get(acopy) _outactors))) 2e+02)) (+ (.y (Transformation|GetWorldLocation (Variables|/Game/RogueLike_Game/Character/Player/Widgets/MapMenu/MapMenu_CameraActor.MapMenu_CameraActor_C|GetDefaultSceneRoot (Utilities|Array|Get(acopy) _outactors)))) (/ (Variables|/Script/Engine.SceneCaptureComponent2D|GetOrthoWidth (Variables|/Game/RogueLike_Game/Character/Player/Widgets/MapMenu/MapMenu_CameraActor.MapMenu_CameraActor_C|GetMapMenu_ComponentCapture (Utilities|Array|Get(acopy) _outactors))) 2e+02)) 0.0) false false)
    (elif (< Axis_X_Value 0.0)
      (Transformation|SetWorldLocation (Variables|/Game/RogueLike_Game/Character/Player/Widgets/MapMenu/MapMenu_CameraActor.MapMenu_CameraActor_C|GetDefaultSceneRoot (Utilities|Array|Get(acopy) _outactors)) (Math|Vector|MakeVector (- (.x (Transformation|GetWorldLocation (Variables|/Game/RogueLike_Game/Character/Player/Widgets/MapMenu/MapMenu_CameraActor.MapMenu_CameraActor_C|GetDefaultSceneRoot (Utilities|Array|Get(acopy) _outactors)))) (/ (Variables|/Script/Engine.SceneCaptureComponent2D|GetOrthoWidth (Variables|/Game/RogueLike_Game/Character/Player/Widgets/MapMenu/MapMenu_CameraActor.MapMenu_CameraActor_C|GetMapMenu_ComponentCapture (Utilities|Array|Get(acopy) _outactors))) 2e+02)) (- (.y (Transformation|GetWorldLocation (Variables|/Game/RogueLike_Game/Character/Player/Widgets/MapMenu/MapMenu_CameraActor.MapMenu_CameraActor_C|GetDefaultSceneRoot (Utilities|Array|Get(acopy) _outactors)))) (/ (Variables|/Script/Engine.SceneCaptureComponent2D|GetOrthoWidth (Variables|/Game/RogueLike_Game/Character/Player/Widgets/MapMenu/MapMenu_CameraActor.MapMenu_CameraActor_C|GetMapMenu_ComponentCapture (Utilities|Array|Get(acopy) _outactors))) 2e+02)) 0.0) false false))))

(fn MoveMapMenuYAxis
  (params (Axis_Y_Value :type Float%20%28single-precision%29))
  (bind _outactors (Actor|GetAllActorsOfClass "/Game/RogueLike_Game/Character/Player/Widgets/MapMenu/MapMenu_CameraActor.MapMenu_CameraActor_C"))
  (if (> Axis_Y_Value 0.0)
    (Transformation|SetWorldLocation (Variables|/Game/RogueLike_Game/Character/Player/Widgets/MapMenu/MapMenu_CameraActor.MapMenu_CameraActor_C|GetDefaultSceneRoot (Utilities|Array|Get(acopy) _outactors)) (Math|Vector|MakeVector (- (.x (Transformation|GetWorldLocation (Variables|/Game/RogueLike_Game/Character/Player/Widgets/MapMenu/MapMenu_CameraActor.MapMenu_CameraActor_C|GetDefaultSceneRoot (Utilities|Array|Get(acopy) _outactors)))) (/ (Variables|/Script/Engine.SceneCaptureComponent2D|GetOrthoWidth (Variables|/Game/RogueLike_Game/Character/Player/Widgets/MapMenu/MapMenu_CameraActor.MapMenu_CameraActor_C|GetMapMenu_ComponentCapture (Utilities|Array|Get(acopy) _outactors))) 2e+02)) (+ (.y (Transformation|GetWorldLocation (Variables|/Game/RogueLike_Game/Character/Player/Widgets/MapMenu/MapMenu_CameraActor.MapMenu_CameraActor_C|GetDefaultSceneRoot (Utilities|Array|Get(acopy) _outactors)))) (/ (Variables|/Script/Engine.SceneCaptureComponent2D|GetOrthoWidth (Variables|/Game/RogueLike_Game/Character/Player/Widgets/MapMenu/MapMenu_CameraActor.MapMenu_CameraActor_C|GetMapMenu_ComponentCapture (Utilities|Array|Get(acopy) _outactors))) 2e+02)) 0.0) false false)
    (elif (< Axis_Y_Value 0.0)
      (Transformation|SetWorldLocation (Variables|/Game/RogueLike_Game/Character/Player/Widgets/MapMenu/MapMenu_CameraActor.MapMenu_CameraActor_C|GetDefaultSceneRoot (Utilities|Array|Get(acopy) _outactors)) (Math|Vector|MakeVector (+ (.x (Transformation|GetWorldLocation (Variables|/Game/RogueLike_Game/Character/Player/Widgets/MapMenu/MapMenu_CameraActor.MapMenu_CameraActor_C|GetDefaultSceneRoot (Utilities|Array|Get(acopy) _outactors)))) (/ (Variables|/Script/Engine.SceneCaptureComponent2D|GetOrthoWidth (Variables|/Game/RogueLike_Game/Character/Player/Widgets/MapMenu/MapMenu_CameraActor.MapMenu_CameraActor_C|GetMapMenu_ComponentCapture (Utilities|Array|Get(acopy) _outactors))) 2e+02)) (- (.y (Transformation|GetWorldLocation (Variables|/Game/RogueLike_Game/Character/Player/Widgets/MapMenu/MapMenu_CameraActor.MapMenu_CameraActor_C|GetDefaultSceneRoot (Utilities|Array|Get(acopy) _outactors)))) (/ (Variables|/Script/Engine.SceneCaptureComponent2D|GetOrthoWidth (Variables|/Game/RogueLike_Game/Character/Player/Widgets/MapMenu/MapMenu_CameraActor.MapMenu_CameraActor_C|GetMapMenu_ComponentCapture (Utilities|Array|Get(acopy) _outactors))) 2e+02)) 0.0) false false))))