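; Player character for the roguelike prototype, with diagonal-axis movement, cursor facing outside the hub, interaction input and an inventory toggle.
; Outside the hub it opens a map menu that redirects input to pan, zoom and recenter an orthographic capture actor, and supports teleporting to map points.
; A per-tick forward sphere trace highlights chests and loot.
; Helper functions total helmet and chestplate stats, then derive walk speed and max health.
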(event Custom|Teleport_From_Map
  ;[1 1 1] Map_Teleportation
  (Widget|RemovefromParent (Variables|Map_Menu|GetMapMenu_Widget))
  (Variables|Conditions|SetMapMenu%20Open? false)
  (Utilities|FlowControl|Sequence
    (:then_0
      (Utilities|FlowControl|Delay 0.1)
      (bind _returnvalue (UserInterface|CreateWidget "/Game/RogueLike_Game/Proto/Characters/Player/Widgets/Teleport_HUD.Teleport_HUD_C"))
      (UserInterface|Viewport|AddtoViewport _returnvalue 0)
      (Utilities|FlowControl|Delay 0.75)
      (Widget|RemovefromParent _returnvalue))
    (:then_1
      (Utilities|FlowControl|Delay 0.2)
      (bind _outactors (Actor|GetAllActorsOfClass "/Game/RogueLike_Game/Proto/Characters/Player/Widgets/MapMenu/Blueprints/MapMenu_Camera_Actor.MapMenu_Camera_Actor_C"))
      (Rendering|SetCustomDepthStencilValue (Variables|/Game/RogueLike_Game/Proto/Characters/Player/Widgets/MapMenu/Blueprints/MapMenu_Camera_Actor.MapMenu_Camera_Actor_C|GetCurrent_Hit_Component (Utilities|Array|Get(acopy) _outactors)) (Variables|/Game/RogueLike_Game/Proto/Characters/Player/Widgets/MapMenu/Blueprints/MapMenu_Camera_Actor.MapMenu_Camera_Actor_C|GetCurrent_Stencil_Value_Component (Utilities|Array|Get(acopy) _outactors)))
      (Transformation|SetWorldLocation (Variables|Collision|GetCapsuleComponent) (Math|Vector|MakeVector (.x (Transformation|GetWorldLocation (Variables|/Game/RogueLike_Game/Proto/Characters/Player/Widgets/MapMenu/Blueprints/MapMenu_Camera_Actor.MapMenu_Camera_Actor_C|GetCurrent_Hit_Component (Utilities|Array|Get(acopy) _outactors)))) (.y (Transformation|GetWorldLocation (Variables|/Game/RogueLike_Game/Proto/Characters/Player/Widgets/MapMenu/Blueprints/MapMenu_Camera_Actor.MapMenu_Camera_Actor_C|GetCurrent_Hit_Component (Utilities|Array|Get(acopy) _outactors)))) 95.0) false false))))

(event EventTick
  (params (DeltaSeconds :type Float%20%28single-precision%29))
  (Utilities|FlowControl|Sequence
    (:then_0
      (CallFunction|HighlightObject))))

(event Input|ActionEvents|InputActionOpen_MapMenu
  (params (Key :type Key%20Structure))
  (bind _returnvalue (Transformation|GetActorLocation))
  ;[1 1 1] Open_Map
  (:Pressed
    (if (not (Variables|Conditions|GetIs%20in%20HUB?))
      (if (Variables|Conditions|GetMapMenu%20Open?)
        (Widget|RemovefromParent (Variables|Map_Menu|GetMapMenu_Widget))
        (Variables|Conditions|SetMapMenu%20Open? false)
        (else
          (bind _returnvalue_2 (UserInterface|CreateWidget "/Game/RogueLike_Game/Proto/Characters/Player/Widgets/MapMenu/Widgets/MapMenu_Widget.MapMenu_Widget_C"))
          (bind _output_get (Variables|Map_Menu|SetMapMenu_Widget _returnvalue_2))
          (UserInterface|Viewport|AddtoViewport _output_get 0)
          (Variables|Conditions|SetMapMenu%20Open? true)
          (bind _returnvalue_3 (Actor|GetActorOfClass "/Game/RogueLike_Game/Proto/Characters/Player/Widgets/MapMenu/Blueprints/MapMenu_Camera_Actor.MapMenu_Camera_Actor_C"))
          (Transformation|SetWorldLocation (Variables|/Game/RogueLike_Game/Proto/Characters/Player/Widgets/MapMenu/Blueprints/MapMenu_Camera_Actor.MapMenu_Camera_Actor_C|GetDefaultSceneRoot _returnvalue_3) (Math|Vector|MakeVector (.x _returnvalue) (.y _returnvalue) -1e+03) false false))))))

(event Input|ActionEvents|InputActionInteraction
  (params (Key :type Key%20Structure))
  (:Pressed
    (Variables|Conditions|SetInteract? true))
  (:Released
    (Variables|Conditions|SetInteract? false)))

(event Input|ActionEvents|InputActionInventory_Menu
  (params (Key :type Key%20Structure))
  (:Pressed
    (if (Variables|Conditions|GetInventory_Open?)
      (Widget|RemovefromParent (stale _returnvalue))
      (Variables|Conditions|SetInventory_Open? false)
      (else
        (bind _returnvalue (UserInterface|CreateWidget "/Game/RogueLike_Game/Proto/Characters/Player/Widgets/Inventaire/Inventory_Widget.Inventory_Widget_C"))
        (UserInterface|Viewport|AddtoViewport _returnvalue 0)
        (Variables|Conditions|SetInventory_Open? true)))))

(event Input|ActionEvents|InputActionRecenter_Map_Menu
  (params (Key :type Key%20Structure))
  (bind _returnvalue (Transformation|GetActorLocation))
  ;[1 1 1] Recenter_MapMenu
  (:Pressed
    (if (Variables|Conditions|GetMapMenu%20Open?)
      (bind _outactors (Actor|GetAllActorsOfClass "/Game/RogueLike_Game/Proto/Characters/Player/Widgets/MapMenu/Blueprints/MapMenu_Camera_Actor.MapMenu_Camera_Actor_C"))
      (Transformation|SetWorldLocation (Variables|/Game/RogueLike_Game/Proto/Characters/Player/Widgets/MapMenu/Blueprints/MapMenu_Camera_Actor.MapMenu_Camera_Actor_C|GetDefaultSceneRoot (Utilities|Array|Get(acopy) _outactors)) (Math|Vector|MakeVector (.x _returnvalue) (.y _returnvalue) -1e+03) false false))))

(event Input|AxisEvents|InputAxisMoveForward
  (params (AxisValue :type Float%20%28single-precision%29))
  (bind _returnvalue (* AxisValue 1e+02))
  (if (Variables|Conditions|GetCan_Move?)
    (if (Variables|Conditions|GetMapMenu%20Open?)
      (CallFunction|MoveMapMenuXAxis AxisValue)
      (else
        (Pawn|Input|AddMovementInput (Math|Vector|MakeVector _returnvalue _returnvalue 0.0) 1.0 false)
        (CallFunction|CharacterLookatCursor)))))

(event Input|AxisEvents|InputAxisMoveRight
  (params (AxisValue :type Float%20%28single-precision%29))
  (bind _returnvalue (* AxisValue 1e+02))
  (if (Variables|Conditions|GetCan_Move?)
    (if (Variables|Conditions|GetMapMenu%20Open?)
      (CallFunction|MoveMapMenuYAxis AxisValue)
      (else
        (Pawn|Input|AddMovementInput (Math|Vector|MakeVector (* _returnvalue -1.0) _returnvalue 0.0) 1.0 false)
        (CallFunction|CharacterLookatCursor)))))

(event Input|AxisEvents|InputAxisLeftClick_Hold
  (params (AxisValue :type Float%20%28single-precision%29))
  (bind _returnvalue (Class|Actor|GetInputAxisKeyValue))
  (bind _returnvalue_2 (Class|Actor|GetInputAxisKeyValue))
  ;[1 1 1] Drag MapMenu
  (if (Variables|Conditions|GetMapMenu%20Open?)
    (bind _outactors (Actor|GetAllActorsOfClass "/Game/RogueLike_Game/Proto/Characters/Player/Widgets/MapMenu/Blueprints/MapMenu_Camera_Actor.MapMenu_Camera_Actor_C"))
    (if (> _returnvalue 0.0)
      (Transformation|SetWorldLocation (Variables|/Game/RogueLike_Game/Proto/Characters/Player/Widgets/MapMenu/Blueprints/MapMenu_Camera_Actor.MapMenu_Camera_Actor_C|GetDefaultSceneRoot (Utilities|Array|Get(acopy) _outactors)) (Math|Vector|MakeVector (+ (.x (Transformation|GetWorldLocation (Variables|/Game/RogueLike_Game/Proto/Characters/Player/Widgets/MapMenu/Blueprints/MapMenu_Camera_Actor.MapMenu_Camera_Actor_C|GetDefaultSceneRoot (Utilities|Array|Get(acopy) _outactors)))) (* (/ (Variables|/Script/Engine.SceneCaptureComponent2D|GetOrthoWidth (Variables|/Game/RogueLike_Game/Proto/Characters/Player/Widgets/MapMenu/Blueprints/MapMenu_Camera_Actor.MapMenu_Camera_Actor_C|GetMapMenu_ComponentCapture (Utilities|Array|Get(acopy) _outactors))) 1e+02) (* (Math|Float|Absolute(Float) _returnvalue) -1.0))) (+ (.y (Transformation|GetWorldLocation (Variables|/Game/RogueLike_Game/Proto/Characters/Player/Widgets/MapMenu/Blueprints/MapMenu_Camera_Actor.MapMenu_Camera_Actor_C|GetDefaultSceneRoot (Utilities|Array|Get(acopy) _outactors)))) (* (/ (Variables|/Script/Engine.SceneCaptureComponent2D|GetOrthoWidth (Variables|/Game/RogueLike_Game/Proto/Characters/Player/Widgets/MapMenu/Blueprints/MapMenu_Camera_Actor.MapMenu_Camera_Actor_C|GetMapMenu_ComponentCapture (Utilities|Array|Get(acopy) _outactors))) 1e+02) (* (Math|Float|Absolute(Float) _returnvalue) -1.0))) -1e+03) false false)
      (elif (< _returnvalue 0.0)
        (Transformation|SetWorldLocation (Variables|/Game/RogueLike_Game/Proto/Characters/Player/Widgets/MapMenu/Blueprints/MapMenu_Camera_Actor.MapMenu_Camera_Actor_C|GetDefaultSceneRoot (Utilities|Array|Get(acopy) _outactors)) (Math|Vector|MakeVector (- (.x (Transformation|GetWorldLocation (Variables|/Game/RogueLike_Game/Proto/Characters/Player/Widgets/MapMenu/Blueprints/MapMenu_Camera_Actor.MapMenu_Camera_Actor_C|GetDefaultSceneRoot (Utilities|Array|Get(acopy) _outactors)))) (* (/ (Variables|/Script/Engine.SceneCaptureComponent2D|GetOrthoWidth (Variables|/Game/RogueLike_Game/Proto/Characters/Player/Widgets/MapMenu/Blueprints/MapMenu_Camera_Actor.MapMenu_Camera_Actor_C|GetMapMenu_ComponentCapture (Utilities|Array|Get(acopy) _outactors))) 1e+02) (* (Math|Float|Absolute(Float) _returnvalue) -1.0))) (- (.y (Transformation|GetWorldLocation (Variables|/Game/RogueLike_Game/Proto/Characters/Player/Widgets/MapMenu/Blueprints/MapMenu_Camera_Actor.MapMenu_Camera_Actor_C|GetDefaultSceneRoot (Utilities|Array|Get(acopy) _outactors)))) (* (/ (Variables|/Script/Engine.SceneCaptureComponent2D|GetOrthoWidth (Variables|/Game/RogueLike_Game/Proto/Characters/Player/Widgets/MapMenu/Blueprints/MapMenu_Camera_Actor.MapMenu_Camera_Actor_C|GetMapMenu_ComponentCapture (Utilities|Array|Get(acopy) _outactors))) 1e+02) (* (Math|Float|Absolute(Float) _returnvalue) -1.0))) -1e+03) false false)))
    (if (< _returnvalue_2 0.0)
      (Transformation|SetWorldLocation (Variables|/Game/RogueLike_Game/Proto/Characters/Player/Widgets/MapMenu/Blueprints/MapMenu_Camera_Actor.MapMenu_Camera_Actor_C|GetDefaultSceneRoot (Utilities|Array|Get(acopy) _outactors)) (Math|Vector|MakeVector (- (.x (Transformation|GetWorldLocation (Variables|/Game/RogueLike_Game/Proto/Characters/Player/Widgets/MapMenu/Blueprints/MapMenu_Camera_Actor.MapMenu_Camera_Actor_C|GetDefaultSceneRoot (Utilities|Array|Get(acopy) _outactors)))) (* (/ (Variables|/Script/Engine.SceneCaptureComponent2D|GetOrthoWidth (Variables|/Game/RogueLike_Game/Proto/Characters/Player/Widgets/MapMenu/Blueprints/MapMenu_Camera_Actor.MapMenu_Camera_Actor_C|GetMapMenu_ComponentCapture (Utilities|Array|Get(acopy) _outactors))) 1e+02) (Math|Float|Absolute(Float) _returnvalue_2))) (+ (.y (Transformation|GetWorldLocation (Variables|/Game/RogueLike_Game/Proto/Characters/Player/Widgets/MapMenu/Blueprints/MapMenu_Camera_Actor.MapMenu_Camera_Actor_C|GetDefaultSceneRoot (Utilities|Array|Get(acopy) _outactors)))) (* (/ (Variables|/Script/Engine.SceneCaptureComponent2D|GetOrthoWidth (Variables|/Game/RogueLike_Game/Proto/Characters/Player/Widgets/MapMenu/Blueprints/MapMenu_Camera_Actor.MapMenu_Camera_Actor_C|GetMapMenu_ComponentCapture (Utilities|Array|Get(acopy) _outactors))) 1e+02) (Math|Float|Absolute(Float) _returnvalue_2))) -1e+03) false false)
      (elif (> _returnvalue_2 0.0)
        (Transformation|SetWorldLocation (Variables|/Game/RogueLike_Game/Proto/Characters/Player/Widgets/MapMenu/Blueprints/MapMenu_Camera_Actor.MapMenu_Camera_Actor_C|GetDefaultSceneRoot (Utilities|Array|Get(acopy) _outactors)) (Math|Vector|MakeVector (+ (.x (Transformation|GetWorldLocation (Variables|/Game/RogueLike_Game/Proto/Characters/Player/Widgets/MapMenu/Blueprints/MapMenu_Camera_Actor.MapMenu_Camera_Actor_C|GetDefaultSceneRoot (Utilities|Array|Get(acopy) _outactors)))) (* (/ (Variables|/Script/Engine.SceneCaptureComponent2D|GetOrthoWidth (Variables|/Game/RogueLike_Game/Proto/Characters/Player/Widgets/MapMenu/Blueprints/MapMenu_Camera_Actor.MapMenu_Camera_Actor_C|GetMapMenu_ComponentCapture (Utilities|Array|Get(acopy) _outactors))) 1e+02) (Math|Float|Absolute(Float) _returnvalue_2))) (- (.y (Transformation|GetWorldLocation (Variables|/Game/RogueLike_Game/Proto/Characters/Player/Widgets/MapMenu/Blueprints/MapMenu_Camera_Actor.MapMenu_Camera_Actor_C|GetDefaultSceneRoot (Utilities|Array|Get(acopy) _outactors)))) (* (/ (Variables|/Script/Engine.SceneCaptureComponent2D|GetOrthoWidth (Variables|/Game/RogueLike_Game/Proto/Characters/Player/Widgets/MapMenu/Blueprints/MapMenu_Camera_Actor.MapMenu_Camera_Actor_C|GetMapMenu_ComponentCapture (Utilities|Array|Get(acopy) _outactors))) 1e+02) (Math|Float|Absolute(Float) _returnvalue_2))) -1e+03) false false)))))

(event Input|GamepadEvents|GamepadRightTriggerAxis
  (params (AxisValue :type Float%20%28single-precision%29))
  ;[1 1 1] Zoom In/Out MapMenu
  (if (> AxisValue 0.0)
    (if (Variables|Conditions|GetMapMenu%20Open?)
      (bind _returnvalue (Actor|GetActorOfClass "/Game/RogueLike_Game/Proto/Characters/Player/Widgets/MapMenu/Blueprints/MapMenu_Camera_Actor.MapMenu_Camera_Actor_C"))
      (if (> (Variables|/Script/Engine.SceneCaptureComponent2D|GetOrthoWidth (Variables|/Game/RogueLike_Game/Proto/Characters/Player/Widgets/MapMenu/Blueprints/MapMenu_Camera_Actor.MapMenu_Camera_Actor_C|GetMapMenu_ComponentCapture _returnvalue)) (Variables|Map_Menu|GetMin_MapMenu_Zoom))
        (Variables|/Script/Engine.SceneCaptureComponent2D|SetOrthoWidth (Variables|/Game/RogueLike_Game/Proto/Characters/Player/Widgets/MapMenu/Blueprints/MapMenu_Camera_Actor.MapMenu_Camera_Actor_C|GetMapMenu_ComponentCapture _returnvalue) (- (Variables|/Script/Engine.SceneCaptureComponent2D|GetOrthoWidth (Variables|/Game/RogueLike_Game/Proto/Characters/Player/Widgets/MapMenu/Blueprints/MapMenu_Camera_Actor.MapMenu_Camera_Actor_C|GetMapMenu_ComponentCapture _returnvalue)) 5e+03))))))

(event Input|GamepadEvents|GamepadLeftTriggerAxis
  (params (AxisValue :type Float%20%28single-precision%29))
  ;[1 1 1] Zoom In/Out MapMenu
  (if (> AxisValue 0.0)
    (if (Variables|Conditions|GetMapMenu%20Open?)
      (bind _returnvalue (Actor|GetActorOfClass "/Game/RogueLike_Game/Proto/Characters/Player/Widgets/MapMenu/Blueprints/MapMenu_Camera_Actor.MapMenu_Camera_Actor_C"))
      (if (< (Variables|/Script/Engine.SceneCaptureComponent2D|GetOrthoWidth (Variables|/Game/RogueLike_Game/Proto/Characters/Player/Widgets/MapMenu/Blueprints/MapMenu_Camera_Actor.MapMenu_Camera_Actor_C|GetMapMenu_ComponentCapture _returnvalue)) (Variables|Map_Menu|GetMax_MapMenu_Zoom))
        (Variables|/Script/Engine.SceneCaptureComponent2D|SetOrthoWidth (Variables|/Game/RogueLike_Game/Proto/Characters/Player/Widgets/MapMenu/Blueprints/MapMenu_Camera_Actor.MapMenu_Camera_Actor_C|GetMapMenu_ComponentCapture _returnvalue) (+ (Variables|/Script/Engine.SceneCaptureComponent2D|GetOrthoWidth (Variables|/Game/RogueLike_Game/Proto/Characters/Player/Widgets/MapMenu/Blueprints/MapMenu_Camera_Actor.MapMenu_Camera_Actor_C|GetMapMenu_ComponentCapture _returnvalue)) 5e+03))))))

(event Input|MouseEvents|MouseWheelUp
  (params (Key :type Key%20Structure))
  ;[1 1 1] Zoom In/Out MapMenu
  (:Pressed
    (if (Variables|Conditions|GetMapMenu%20Open?)
      (bind _returnvalue (Actor|GetActorOfClass "/Game/RogueLike_Game/Proto/Characters/Player/Widgets/MapMenu/Blueprints/MapMenu_Camera_Actor.MapMenu_Camera_Actor_C"))
      (if (> (Variables|/Script/Engine.SceneCaptureComponent2D|GetOrthoWidth (Variables|/Game/RogueLike_Game/Proto/Characters/Player/Widgets/MapMenu/Blueprints/MapMenu_Camera_Actor.MapMenu_Camera_Actor_C|GetMapMenu_ComponentCapture _returnvalue)) (Variables|Map_Menu|GetMin_MapMenu_Zoom))
        (Variables|/Script/Engine.SceneCaptureComponent2D|SetOrthoWidth (Variables|/Game/RogueLike_Game/Proto/Characters/Player/Widgets/MapMenu/Blueprints/MapMenu_Camera_Actor.MapMenu_Camera_Actor_C|GetMapMenu_ComponentCapture _returnvalue) (- (Variables|/Script/Engine.SceneCaptureComponent2D|GetOrthoWidth (Variables|/Game/RogueLike_Game/Proto/Characters/Player/Widgets/MapMenu/Blueprints/MapMenu_Camera_Actor.MapMenu_Camera_Actor_C|GetMapMenu_ComponentCapture _returnvalue)) 5e+03))))))

(event Input|MouseEvents|MouseWheelDown
  (params (Key :type Key%20Structure))
  ;[1 1 1] Zoom In/Out MapMenu
  (:Pressed
    (if (Variables|Conditions|GetMapMenu%20Open?)
      (bind _returnvalue (Actor|GetActorOfClass "/Game/RogueLike_Game/Proto/Characters/Player/Widgets/MapMenu/Blueprints/MapMenu_Camera_Actor.MapMenu_Camera_Actor_C"))
      (if (< (Variables|/Script/Engine.SceneCaptureComponent2D|GetOrthoWidth (Variables|/Game/RogueLike_Game/Proto/Characters/Player/Widgets/MapMenu/Blueprints/MapMenu_Camera_Actor.MapMenu_Camera_Actor_C|GetMapMenu_ComponentCapture _returnvalue)) (Variables|Map_Menu|GetMax_MapMenu_Zoom))
        (Variables|/Script/Engine.SceneCaptureComponent2D|SetOrthoWidth (Variables|/Game/RogueLike_Game/Proto/Characters/Player/Widgets/MapMenu/Blueprints/MapMenu_Camera_Actor.MapMenu_Camera_Actor_C|GetMapMenu_ComponentCapture _returnvalue) (+ (Variables|/Script/Engine.SceneCaptureComponent2D|GetOrthoWidth (Variables|/Game/RogueLike_Game/Proto/Characters/Player/Widgets/MapMenu/Blueprints/MapMenu_Camera_Actor.MapMenu_Camera_Actor_C|GetMapMenu_ComponentCapture _returnvalue)) 5e+03))))))

(event Input|GamepadEvents|GamepadFaceButtonRight
  (params (Key :type Key%20Structure))
  ;[1 1 1] Open_Map
  (:Pressed
    (if (Variables|Conditions|GetMapMenu%20Open?)
      (Widget|RemovefromParent (Variables|Map_Menu|GetMapMenu_Widget))
      (Variables|Conditions|SetMapMenu%20Open? false))))

(fn ConstructionScript)

(fn CharacterLookatCursor
  (if (not (Variables|Conditions|GetIs%20in%20HUB?))
    (Transformation|SetWorldRotation (Variables|Collision|GetCapsuleComponent) (Math|Rotator|MakeRotator 0.0 0.0 (.yaw (Math|Rotator|FindLookatRotation (Transformation|GetActorLocation self) (.Location (Collision|BreakHitResult (.HitResult (Game|Player|GetHitResultUnderCursorbyChannel (Game|GetPlayerController 0) "TraceTypeQuery1" true))))))) false false)))

(fn MoveMapMenuXAxis
  (params (Axis_X_Value :type Float%20%28single-precision%29))
  (bind _outactors (Actor|GetAllActorsOfClass "/Game/RogueLike_Game/Proto/Characters/Player/Widgets/MapMenu/Blueprints/MapMenu_Camera_Actor.MapMenu_Camera_Actor_C"))
  (if (> Axis_X_Value 0.0)
    (Transformation|SetWorldLocation (Variables|/Game/RogueLike_Game/Proto/Characters/Player/Widgets/MapMenu/Blueprints/MapMenu_Camera_Actor.MapMenu_Camera_Actor_C|GetDefaultSceneRoot (Utilities|Array|Get(acopy) _outactors)) (Math|Vector|MakeVector (+ (.x (Transformation|GetWorldLocation (Variables|/Game/RogueLike_Game/Proto/Characters/Player/Widgets/MapMenu/Blueprints/MapMenu_Camera_Actor.MapMenu_Camera_Actor_C|GetDefaultSceneRoot (Utilities|Array|Get(acopy) _outactors)))) (/ (Variables|/Script/Engine.SceneCaptureComponent2D|GetOrthoWidth (Variables|/Game/RogueLike_Game/Proto/Characters/Player/Widgets/MapMenu/Blueprints/MapMenu_Camera_Actor.MapMenu_Camera_Actor_C|GetMapMenu_ComponentCapture (Utilities|Array|Get(acopy) _outactors))) 2e+02)) (+ (.y (Transformation|GetWorldLocation (Variables|/Game/RogueLike_Game/Proto/Characters/Player/Widgets/MapMenu/Blueprints/MapMenu_Camera_Actor.MapMenu_Camera_Actor_C|GetDefaultSceneRoot (Utilities|Array|Get(acopy) _outactors)))) (/ (Variables|/Script/Engine.SceneCaptureComponent2D|GetOrthoWidth (Variables|/Game/RogueLike_Game/Proto/Characters/Player/Widgets/MapMenu/Blueprints/MapMenu_Camera_Actor.MapMenu_Camera_Actor_C|GetMapMenu_ComponentCapture (Utilities|Array|Get(acopy) _outactors))) 2e+02)) -1e+03) false false)
    (elif (< Axis_X_Value 0.0)
      (Transformation|SetWorldLocation (Variables|/Game/RogueLike_Game/Proto/Characters/Player/Widgets/MapMenu/Blueprints/MapMenu_Camera_Actor.MapMenu_Camera_Actor_C|GetDefaultSceneRoot (Utilities|Array|Get(acopy) _outactors)) (Math|Vector|MakeVector (- (.x (Transformation|GetWorldLocation (Variables|/Game/RogueLike_Game/Proto/Characters/Player/Widgets/MapMenu/Blueprints/MapMenu_Camera_Actor.MapMenu_Camera_Actor_C|GetDefaultSceneRoot (Utilities|Array|Get(acopy) _outactors)))) (/ (Variables|/Script/Engine.SceneCaptureComponent2D|GetOrthoWidth (Variables|/Game/RogueLike_Game/Proto/Characters/Player/Widgets/MapMenu/Blueprints/MapMenu_Camera_Actor.MapMenu_Camera_Actor_C|GetMapMenu_ComponentCapture (Utilities|Array|Get(acopy) _outactors))) 2e+02)) (- (.y (Transformation|GetWorldLocation (Variables|/Game/RogueLike_Game/Proto/Characters/Player/Widgets/MapMenu/Blueprints/MapMenu_Camera_Actor.MapMenu_Camera_Actor_C|GetDefaultSceneRoot (Utilities|Array|Get(acopy) _outactors)))) (/ (Variables|/Script/Engine.SceneCaptureComponent2D|GetOrthoWidth (Variables|/Game/RogueLike_Game/Proto/Characters/Player/Widgets/MapMenu/Blueprints/MapMenu_Camera_Actor.MapMenu_Camera_Actor_C|GetMapMenu_ComponentCapture (Utilities|Array|Get(acopy) _outactors))) 2e+02)) -1e+03) false false))))

(fn MoveMapMenuYAxis
  (params (Axis_Y_Value :type Float%20%28single-precision%29))
  (bind _outactors (Actor|GetAllActorsOfClass "/Game/RogueLike_Game/Proto/Characters/Player/Widgets/MapMenu/Blueprints/MapMenu_Camera_Actor.MapMenu_Camera_Actor_C"))
  (if (> Axis_Y_Value 0.0)
    (Transformation|SetWorldLocation (Variables|/Game/RogueLike_Game/Proto/Characters/Player/Widgets/MapMenu/Blueprints/MapMenu_Camera_Actor.MapMenu_Camera_Actor_C|GetDefaultSceneRoot (Utilities|Array|Get(acopy) _outactors)) (Math|Vector|MakeVector (- (.x (Transformation|GetWorldLocation (Variables|/Game/RogueLike_Game/Proto/Characters/Player/Widgets/MapMenu/Blueprints/MapMenu_Camera_Actor.MapMenu_Camera_Actor_C|GetDefaultSceneRoot (Utilities|Array|Get(acopy) _outactors)))) (/ (Variables|/Script/Engine.SceneCaptureComponent2D|GetOrthoWidth (Variables|/Game/RogueLike_Game/Proto/Characters/Player/Widgets/MapMenu/Blueprints/MapMenu_Camera_Actor.MapMenu_Camera_Actor_C|GetMapMenu_ComponentCapture (Utilities|Array|Get(acopy) _outactors))) 2e+02)) (+ (.y (Transformation|GetWorldLocation (Variables|/Game/RogueLike_Game/Proto/Characters/Player/Widgets/MapMenu/Blueprints/MapMenu_Camera_Actor.MapMenu_Camera_Actor_C|GetDefaultSceneRoot (Utilities|Array|Get(acopy) _outactors)))) (/ (Variables|/Script/Engine.SceneCaptureComponent2D|GetOrthoWidth (Variables|/Game/RogueLike_Game/Proto/Characters/Player/Widgets/MapMenu/Blueprints/MapMenu_Camera_Actor.MapMenu_Camera_Actor_C|GetMapMenu_ComponentCapture (Utilities|Array|Get(acopy) _outactors))) 2e+02)) -1e+03) false false)
    (elif (< Axis_Y_Value 0.0)
      (Transformation|SetWorldLocation (Variables|/Game/RogueLike_Game/Proto/Characters/Player/Widgets/MapMenu/Blueprints/MapMenu_Camera_Actor.MapMenu_Camera_Actor_C|GetDefaultSceneRoot (Utilities|Array|Get(acopy) _outactors)) (Math|Vector|MakeVector (+ (.x (Transformation|GetWorldLocation (Variables|/Game/RogueLike_Game/Proto/Characters/Player/Widgets/MapMenu/Blueprints/MapMenu_Camera_Actor.MapMenu_Camera_Actor_C|GetDefaultSceneRoot (Utilities|Array|Get(acopy) _outactors)))) (/ (Variables|/Script/Engine.SceneCaptureComponent2D|GetOrthoWidth (Variables|/Game/RogueLike_Game/Proto/Characters/Player/Widgets/MapMenu/Blueprints/MapMenu_Camera_Actor.MapMenu_Camera_Actor_C|GetMapMenu_ComponentCapture (Utilities|Array|Get(acopy) _outactors))) 2e+02)) (- (.y (Transformation|GetWorldLocation (Variables|/Game/RogueLike_Game/Proto/Characters/Player/Widgets/MapMenu/Blueprints/MapMenu_Camera_Actor.MapMenu_Camera_Actor_C|GetDefaultSceneRoot (Utilities|Array|Get(acopy) _outactors)))) (/ (Variables|/Script/Engine.SceneCaptureComponent2D|GetOrthoWidth (Variables|/Game/RogueLike_Game/Proto/Characters/Player/Widgets/MapMenu/Blueprints/MapMenu_Camera_Actor.MapMenu_Camera_Actor_C|GetMapMenu_ComponentCapture (Utilities|Array|Get(acopy) _outactors))) 2e+02)) -1e+03) false false))))

(fn CheckArmorStatValue
  (bind _returnvalue (Actor|GetActorOfClass "/Game/RogueLike_Game/Proto/Characters/Player/Widgets/Inventaire/Helmet/Helmet_Render_Actor.Helmet_Render_Actor_C"))
  (LocalVariables|SetHelmet_Primary_Stat_Type (Variables|/Game/RogueLike_Game/Proto/Characters/Player/Widgets/Inventaire/Helmet/Helmet_Render_Actor.Helmet_Render_Actor_C|GetPrimary_Stat_Type _returnvalue))
  (LocalVariables|SetHelmet_Primary_Stat_Value (Variables|/Game/RogueLike_Game/Proto/Characters/Player/Widgets/Inventaire/Helmet/Helmet_Render_Actor.Helmet_Render_Actor_C|GetPrimary_Stat_Value _returnvalue))
  (LocalVariables|SetHelmet_Secondary_Stat_Type (Variables|/Game/RogueLike_Game/Proto/Characters/Player/Widgets/Inventaire/Helmet/Helmet_Render_Actor.Helmet_Render_Actor_C|GetSecondary_Stat_Type _returnvalue))
  (if (Variables|/Game/RogueLike_Game/Proto/Characters/Player/Widgets/Inventaire/Helmet/Helmet_Render_Actor.Helmet_Render_Actor_C|GetSecondary_Stat_Negative? _returnvalue)
    (LocalVariables|SetHelmet_Secondary_Stat_Value (* (Variables|/Game/RogueLike_Game/Proto/Characters/Player/Widgets/Inventaire/Helmet/Helmet_Render_Actor.Helmet_Render_Actor_C|GetSecondary_Stat_Value _returnvalue) -1))
    (else
      (LocalVariables|SetHelmet_Secondary_Stat_Value (Variables|/Game/RogueLike_Game/Proto/Characters/Player/Widgets/Inventaire/Helmet/Helmet_Render_Actor.Helmet_Render_Actor_C|GetSecondary_Stat_Value _returnvalue))))
  (bind _returnvalue_2 (Actor|GetActorOfClass "/Game/RogueLike_Game/Proto/Characters/Player/Widgets/Inventaire/ChestPlate/ChestPlate_Render_Actor.ChestPlate_Render_Actor_C"))
  (LocalVariables|SetChestPlate_Primary_Stat_Type (Variables|/Game/RogueLike_Game/Proto/Characters/Player/Widgets/Inventaire/ChestPlate/ChestPlate_Render_Actor.ChestPlate_Render_Actor_C|GetPrimary_Stat_Type _returnvalue_2))
  (LocalVariables|SetChestPlate_Primary_Stat_Value (Variables|/Game/RogueLike_Game/Proto/Characters/Player/Widgets/Inventaire/ChestPlate/ChestPlate_Render_Actor.ChestPlate_Render_Actor_C|GetPrimary_Stat_Value _returnvalue_2))
  (LocalVariables|SetChestPlate_Secondary_Stat_Type (Variables|/Game/RogueLike_Game/Proto/Characters/Player/Widgets/Inventaire/ChestPlate/ChestPlate_Render_Actor.ChestPlate_Render_Actor_C|GetSecondary_Stat_Type _returnvalue_2))
  (if (Variables|/Game/RogueLike_Game/Proto/Characters/Player/Widgets/Inventaire/ChestPlate/ChestPlate_Render_Actor.ChestPlate_Render_Actor_C|GetSecondary_Stat_Negative? _returnvalue_2)
    (LocalVariables|SetChestPlate_Secondary_Stat_Value (* (Variables|/Game/RogueLike_Game/Proto/Characters/Player/Widgets/Inventaire/ChestPlate/ChestPlate_Render_Actor.ChestPlate_Render_Actor_C|GetSecondary_Stat_Value _returnvalue_2) -1))
    (else
      (LocalVariables|SetChestPlate_Secondary_Stat_Value (Variables|/Game/RogueLike_Game/Proto/Characters/Player/Widgets/Inventaire/ChestPlate/ChestPlate_Render_Actor.ChestPlate_Render_Actor_C|GetSecondary_Stat_Value _returnvalue_2))))
  (for (_array_element _array_index) (Variables|Statistics|GetPlayer_Stats_Map)
    (if (Utilities|Enum|Equal(Enum) _array_element (LocalVariables|GetHelmet_Primary_Stat_Type))
      (Utilities|Array|SetArrayElem (Variables|Statistics|GetStatistics_Values) _array_index (LocalVariables|GetHelmet_Primary_Stat_Value))
      (else
        (Utilities|Array|SetArrayElem (Variables|Statistics|GetStatistics_Values) _array_index 0))))
  (for (_array_element_2 _array_index_2) (Variables|Statistics|GetPlayer_Stats_Map)
    (if (Utilities|Enum|Equal(Enum) _array_element_2 (LocalVariables|GetChestPlate_Primary_Stat_Type))
      (Utilities|Array|SetArrayElem (Variables|Statistics|GetStatistics_Values) _array_index_2 (+ (LocalVariables|GetChestPlate_Primary_Stat_Value) (Utilities|Array|Get(acopy) (Variables|Statistics|GetStatistics_Values) _array_index_2)))))
  (for (_array_element_3 _array_index_3) (Variables|Statistics|GetPlayer_Stats_Map)
    (if (Utilities|Enum|Equal(Enum) _array_element_3 (LocalVariables|GetHelmet_Secondary_Stat_Type))
      (Utilities|Array|SetArrayElem (Variables|Statistics|GetStatistics_Values) _array_index_3 (+ (LocalVariables|GetHelmet_Secondary_Stat_Value) (Utilities|Array|Get(acopy) (Variables|Statistics|GetStatistics_Values) _array_index_3)))))
  (for (_array_element_4 _array_index_4) (Variables|Statistics|GetPlayer_Stats_Map)
    (if (Utilities|Enum|Equal(Enum) _array_element_4 (LocalVariables|GetChestPlate_Secondary_Stat_Type))
      (Utilities|Array|SetArrayElem (Variables|Statistics|GetStatistics_Values) _array_index_4 (+ (LocalVariables|GetChestPlate_Secondary_Stat_Value) (Utilities|Array|Get(acopy) (Variables|Statistics|GetStatistics_Values) _array_index_4))))))

(fn StatAffectPlayer
  (Utilities|FlowControl|Sequence
    (:then_0
      (Variables|/Script/Engine.CharacterMovementComponent|SetMaxWalkSpeed (Variables|Character|GetCharacterMovement) (+ (* (Utilities|Array|Get(acopy) (Variables|Statistics|GetStatistics_Values)) 3e+01) 6e+02)))
    (:then_2
      (Variables|Statistics|SetMax_HealthPoint (+ (* (Utilities|Array|Get(acopy) (Variables|Statistics|GetStatistics_Values) 2) 5) 100)))))

(fn HighlightObject
  (bind _returnvalue (Game|GetPlayerCharacter 0))
  (bind _returnvalue_2 (Transformation|GetActorLocation _returnvalue))
  (bind _outhit (Collision|SphereTraceByChannel _returnvalue_2 (+ _returnvalue_2 (* (Math|Vector|GetForwardVector (Variables|Collision|GetCapsuleComponent)) 2e+02)) 5e+01 "TraceTypeQuery1" false 0 "None" true "(R=1.000000,G=0.000000,B=0.000000,A=1.000000)" "(R=0.000000,G=1.000000,B=0.000000,A=1.000000)" 1.0))
  (if (.bBlockingHit (Collision|BreakHitResult _outhit))
    (Utilities|FlowControl|DoOnce false :!label _label
      (:Completed
        (bind _output_get (Variables|Default|SetCurrent_Hited_Actor (Components|GetOwner (.HitComponent (Collision|BreakHitResult _outhit)))))
        (if (Actor|ActorHasTag (Components|GetOwner (.HitComponent (Collision|BreakHitResult _outhit))) "Interactable_Actor")
          (bind _aschest_actor (Utilities|Casting|CastToChest_Actor _output_get)
            (:then
              (Default|StartHighlight _aschest_actor))
            (:CastFailed
              (bind _asloot_system_actor_proto (Utilities|Casting|CastToLoot_System_Actor_Proto (Variables|Default|GetCurrent_Hited_Actor)))
              (Default|StartHighlight _asloot_system_actor_proto))))))
    (else
      (bind _aschest_actor_2 (Utilities|Casting|CastToChest_Actor (Variables|Default|GetCurrent_Hited_Actor))
        (:then
          (Utilities|IsValid _aschest_actor_2
            (:Is%20Valid
              (Default|EndHighlight _aschest_actor_2)
              (goto _label Reset))
            (:Is%20Not%20Valid
              (goto _label Reset))))
        (:CastFailed
          (bind _asloot_system_actor_proto_2 (Utilities|Casting|CastToLoot_System_Actor_Proto (Variables|Default|GetCurrent_Hited_Actor))
            (:then
              (Utilities|IsValid _asloot_system_actor_proto_2
                (:Is%20Valid
                  (Default|EndHighlight _asloot_system_actor_proto_2))
                (:Is%20Not%20Valid
                  (goto _label Reset))))
            (:CastFailed
              (goto _label Reset))))))))